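; LCLevelFinishedUI is an in-world end-of-level display actor with scroll and book elements.
; Its construction script stores the placed location as the end position, derives a start position along the up vector, and sets the bounce-in timeline's play rate.
; One FinishedType value changes the scroll text to announce the Champions' fall and hides the book widget and mesh.
; BounceInTimeline would lerp the actor between those positions, but nothing shown starts it.
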(fn ConstructionScript
  (bind _scrollwidget (Variables|Default|GetScrollWidget))
  (bind _returnvalue (UserInterface|GetUserWidgetObject _scrollwidget))
  (bind _aslcumg_level_complete_scroll (Utilities|Casting|CastToLCUMG_LevelComplete_Scroll _returnvalue))
  ;[1 1 1] Timeline stuff
  (Variables|Default|SetEndPosition (Transformation|GetActorLocation))
  (Variables|Default|SetStartPosition (+ (* (Math|Vector|GetUpVector (Transformation|GetActorRotation)) 2e+02) (Variables|Default|GetEndPosition)))
  (Components|Timeline|SetPlayRate (Variables|Default|GetBounceInTimeline) (Variables|Default|GetBounceInPlayRate))
  (if (Utilities|Enum|Equal(Enum) (Variables|Default|GetFinishedType) "NewEnumerator1")
    (Rendering|Components|TextRender|SetText (Variables|/Game/UI/UMG/LCUMG_LevelComplete_Scroll.LCUMG_LevelComplete_Scroll_C|GetTextFirstRow _aslcumg_level_complete_scroll) "The Champions have")
    (Rendering|Components|TextRender|SetText (Variables|/Game/UI/UMG/LCUMG_LevelComplete_Scroll.LCUMG_LevelComplete_Scroll_C|GetTextSecondRow _aslcumg_level_complete_scroll) "fallen!")
    (Rendering|SetVisibility (Variables|Default|GetBookWidget) false false)))