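; Game mode for a three-champion level game, handling HUD creation, champion spawning, music fades and level completion or failure.
; The default pawn starts at the Warrior-tagged PlayerStart, while Druid and Wizard spawn at theirs, and all three register with the player controller.
; Completion records the time and blends the camera to the goal; failure spawns a finish UI facing the camera, then restarts the level.
; ChampionDied's alive-count and fail logic is disconnected.
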(event EventBeginPlay
  ;[1 1 1] Create HUD
  (bind _returnvalue (UserInterface|CreateWidget "/Game/UI/UMG/LCUMG_PlayerHUD.LCUMG_PlayerHUD_C" (Game|GetPlayerController 0)))
  (bind _output_get (Variables|Default|SetPlayerHUD _returnvalue))
  (UserInterface|Viewport|AddtoViewport _output_get 0)
  (bind _outactors (Actor|GetAllActorsOfClass "/Game/Blueprints/Ingredients/LCGoal.LCGoal_C"))
  (Variables|Default|SetGoalActor (Utilities|Array|Get(acopy) _outactors))
  ;[1 1 1] Level stuff
  (bind _returnvalue_2 (Game|GetCurrentLevelName true))
  (CallFunction|SetCurrentLevel self (Utilities|String|StringToName _returnvalue_2)))

(fn ConstructionScript)

(fn SpawnDefaultPawnfor
  (params (NewPlayer :type Controller%20Object%20Reference) (StartSpot :type Actor%20Object%20Reference))
  (bind _returnvalue (|CallParentFunction NewPlayer StartSpot))
  (LocalVariables|SetSpawnedPawnLocal _returnvalue)
  ;[1 1 1] Find the other spawn points
  (bind _outactors (Actor|GetAllActorsOfClass "/Script/Engine.PlayerStart"))
  (for _array_element _outactors
    (if (Utilities|Name|Equal(Name) (Variables|/Script/Engine.PlayerStart|GetPlayerStartTag _array_element) "Druid")
      (LocalVariables|SetDruidPlayerStartLocal _array_element)
      (elif (Utilities|Name|Equal(Name) (Variables|/Script/Engine.PlayerStart|GetPlayerStartTag _array_element) "Wizard")
        (LocalVariables|SetWizardPlayerStartLocal _array_element))))
  (bind _returnvalue_2 (Game|SpawnActorfromClass "/Game/Blueprints/Character/LCCharacter_Druid.LCCharacter_Druid_C" (Transformation|GetActorTransform (LocalVariables|GetDruidPlayerStartLocal)) "AlwaysSpawn" 0 0))
  (bind _returnvalue_3 (Game|SpawnActorfromClass "/Game/Blueprints/Character/LCCharacter_Wizard.LCCharacter_Wizard_C" (Transformation|GetActorTransform (LocalVariables|GetWizardPlayerStartLocal)) "AlwaysSpawn" 0 0))
  (bind _aslcplayer_controller (Utilities|Casting|CastToLCPlayerController (Game|GetPlayerController 0)))
  (Default|CreatePlayerCamera _aslcplayer_controller)
  (bind _aslccharacter_base (Utilities|Casting|CastToLCCharacterBase (LocalVariables|GetSpawnedPawnLocal)))
  (Default|SetChampionReferences _aslcplayer_controller _aslccharacter_base _returnvalue_3 _returnvalue_2)
  (return (LocalVariables|GetSpawnedPawnLocal)))

(fn LevelComplete
  ;[1 1 1] Set the level time
  (Variables|/Game/Blueprints/Game/LCGameState.LCGameState_C|SetLevelTime (.AsLCGame%20State (Utilities|Casting|CastToLCGameState (Game|GetGameState))) (Utilities|Time|GetGameTimeinSeconds))
  (Default|CallLevelCompleted)
  (Input|DisableInput (Game|Player|GetPlayerPawn 0) (Game|GetPlayerController 0))
  (Widget|RemovefromParent (Variables|Default|GetPlayerHUD))
  (bind _aslcplayer_controller (Utilities|Casting|CastToLCPlayerController (Game|GetPlayerController 0)))
  (Game|Player|SetViewTargetwithBlend _aslcplayer_controller (Variables|Default|GetGoalActor) 3.0 "VTBlend_EaseInOut" 3.0 false)
  (Utilities|Time|SetTimerbyFunctionName (Variables|Default|GetGoalActor) "CreateLevelCompleteUI" 3.0))

(fn ChampionDied)

(fn LevelFail
  (bind _returnvalue (Game|GetPlayerCameraManager 0))
  (bind _returnvalue_2 (Game|GetPlayerController 0))
  (bind _transformcomponent (Variables|/Script/Engine.PlayerCameraManager|GetTransformComponent _returnvalue))
  (bind _returnvalue_3 (Transformation|GetWorldTransform _transformcomponent))
  (bind (_location _rotation _scale) (Math|Transform|BreakTransform _returnvalue_3))
  (bind _returnvalue_4 (Math|Vector|GetForwardVector _rotation))
  (bind _returnvalue_5 (* _returnvalue_4 125.0))
  (bind _returnvalue_6 (+ _location _returnvalue_5))
  (Default|CallLevelFailed)
  (Input|DisableInput _returnvalue_2 _returnvalue_2)
  (Widget|RemovefromParent (Variables|Default|GetPlayerHUD))
  (Game|SpawnActorfromClass "/Game/Blueprints/Game/LCLevelFinishedUI.LCLevelFinishedUI_C" (Math|Transform|MakeTransform _returnvalue_6 (Math|Rotator|FindLookatRotation _returnvalue_6 _location) _scale) "AlwaysSpawn" 0 "NewEnumerator1" 0)
  (Utilities|Time|SetTimerbyFunctionName self "RestartLevel" 6.0))

(fn RestartLevel
  (Game|OpenLevel(byName) (Variables|Default|GetCurrentLevelName)))

(fn ChoosePlayerStart
  (params (Player :type Controller%20Object%20Reference))
  (LocalVariables|SetPlayerLocal Player)
  (bind _outactors (Actor|GetAllActorsOfClass "/Script/Engine.PlayerStart"))
  (bind _array_element (Utilities|Array|ForEachLoopwithBreak _outactors)
    (:LoopBody
      (if (Utilities|Name|Equal(Name) (Variables|/Script/Engine.PlayerStart|GetPlayerStartTag _array_element) "Warrior")
        (LocalVariables|SetPlayerStartLocal _array_element)))
    (:Completed
      (Utilities|IsValid (LocalVariables|GetPlayerStartLocal)
        (:Is%20Valid
          _)
        (:Is%20Not%20Valid
          (bind _returnvalue (|CallParentFunction (LocalVariables|GetPlayerLocal)))
          (LocalVariables|SetPlayerStartLocal _returnvalue)))
      (return (LocalVariables|GetPlayerStartLocal)))))

(fn PlayMusic
  (params (MusicTrack :type Sound%20Base%20Object%20Reference) (FadeInDuration :type Float%20%28single-precision%29) (FadeInVolume :type Float%20%28single-precision%29))
  ;[1 1 1] Comment
  (LocalVariables|SetMusicTrackLocal MusicTrack)
  (LocalVariables|SetFadeInDurationLocal FadeInDuration)
  (LocalVariables|SetFadeInVolumeLocal FadeInVolume)
  ;[1 1 1] Comment
  (Audio|Components|Audio|SetSound (Variables|Default|GetMusicController) (LocalVariables|GetMusicTrackLocal))
  (Audio|Components|Audio|FadeIn (Variables|Default|GetMusicController) (LocalVariables|GetFadeInDurationLocal) (LocalVariables|GetFadeInVolumeLocal) 0.0 :!class /Script/Engine.AudioComponent)
  ;[1 1 1] Comment
  (return true))

(fn SetCurrentLevel
  (params (LevelName :type Name :default "None"))
  (Variables|Default|SetCurrentLevelName LevelName)
  (return true))

(fn StopMusic
  (params (FadeOutDuration :type Float%20%28single-precision%29) (FadeOutVolume :type Float%20%28single-precision%29))
  ;[1 1 1] Comment
  (LocalVariables|SetFadeOutDurationLocal FadeOutDuration)
  (LocalVariables|SetFadeOutVolumeLocal FadeOutVolume)
  ;[1 1 1] Comment
  (Audio|Components|Audio|FadeOut (Variables|Default|GetMusicController) (LocalVariables|GetFadeOutDurationLocal) (LocalVariables|GetFadeOutVolumeLocal) :!class /Script/Engine.AudioComponent)
  ;[1 1 1] Comment
  (return true))