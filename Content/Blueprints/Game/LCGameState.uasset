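; LCGameState is a game state Blueprint that tracks champion deaths, enemy kills and a flawless flag.
; It decrements the alive champion count, returning the new number and whether all champions are dead.
; Death recording casts the character to Druid, Warrior or Wizard to set that champion's dead flag, counting any other character as a dead enemy.
; A simple setter stores the flawless stat.
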(fn ConstructionScript)

(fn DecrementAliveChampionCount
  (bind _output_get (Variables|Default|SetAliveChampionCount (- (Variables|Default|GetAliveChampionCount) 1)))
  (return _output_get (== _output_get 0)))

(fn IncrementCharacterDiedStat
  (params (Character :type LC%20Character%20Base%20Object%20Reference))
  (Utilities|Casting|CastToLCCharacter_Druid Character
    (:then
      (Variables|Default|SetDruidDead true))
    (:CastFailed
      (Utilities|Casting|CastToLCCharacter_Warrior Character
        (:then
          (Variables|Default|SetWarriorDead true))
        (:CastFailed
          (Utilities|Casting|CastToLCCharacter_Wizard Character
            (:then
              (Variables|Default|SetWizardDead true))
            (:CastFailed
              (Variables|Default|SetDeadEnemies (+ (Variables|Default|GetDeadEnemies) 1)))))))))

(fn SetFlawlessStat
  (params (Flawless :type Boolean))
  (Variables|Default|SetFlawless Flawless))