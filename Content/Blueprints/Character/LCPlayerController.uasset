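; Player controller that lets the player cycle through three champions (Warrior, Wizard, Druid) and possess the selected one.
; It spawns a shared camera attached to itself, handling look, zoom and an intro rotation timeline with input disabled.
; Switching preserves control rotation and glides the camera to the new champion via timeline.
; Dead champions leave the cycle list without triggering an automatic switch; restart and quit inputs are also handled.
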(event Custom|PlayCamToCharAnimation
  (params (CameraFocus :type Actor%20Object%20Reference))
  (bind _gamecamera (Variables|Default|GetGameCamera))
  ;[1 1 1] Move cam to next char
  (bind _0_1 (Timeline|CamToCharTimeline PlayFromStart)
    (:Update
      (Utilities|IsValid _gamecamera
        (:Is%20Valid
          (Utilities|IsValid CameraFocus
            (:Is%20Valid
              (Transformation|SetActorLocation (Variables|Default|GetGameCamera) (Math|Vector|Lerp(Vector) (Transformation|GetActorLocation _gamecamera) (Transformation|GetActorLocation CameraFocus) _0_1) false false))))))))

(event Custom|MonitorCharacterDeath
  ;[1 1 1] Character has died, remove them from the list
  (for _array_element (Variables|Default|GetCharacterList)
    (EventDispatchers|AssignOnCharacterDied (.AsLCCharacter%20Base (Utilities|Casting|CastToLCCharacterBase _array_element)) (delegate Custom|ChampionHasDied))))

(event Custom|PlayIntroCamAnimation
  (bind _returnvalue (Pawn|GetControlledPawn))
  (bind _self self)
  (bind _self_2 self)
  (bind _returnvalue_2 (Transformation|GetActorRotation _returnvalue))
  ;[1 1 1] Intro cam animation
  (Input|DisableInput _self_2 _self_2)
  (bind _rotation (Timeline|IntroCamTimeline PlayFromStart)
    (:Update
      (Pawn|SetControlRotation (Math|Rotator|Lerp(Rotator) (Math|Rotator|CombineRotators _returnvalue_2 "0,180.000000, 0") (Math|Rotator|CombineRotators _returnvalue_2 "0.000000,0.000000,-30.000000") _rotation)))
    (:Finished
      ;[1 1 1] Reenable input
      (Input|EnableInput _self _self))))

(event Custom|ChampionHasDied
  (params (CharacterWhoDied :type LC%20Character%20Base%20Object%20Reference))
  ;[1 1 1] Character has died, remove them from the list
  (Utilities|Array|RemoveItem (Variables|Default|GetCharacterList) CharacterWhoDied)
  (if (== CharacterWhoDied (Variables|Default|GetCurrentCharacter))
    _))

(event EventBeginPlay
  ;[1 1 1] Create the player's camera
  (CallFunction|CreatePlayerCamera)
  (CallFunction|MonitorCharacterDeath)
  ;[1 1 1] Play the cam
  (CallFunction|PlayIntroCamAnimation))

(event Input|ActionEvents|InputActionRestartLevel
  (params (Key :type Key%20Structure))
  ;[1 1 1] Restart the level
  (:Pressed
    (bind _aslcgame_mode (Utilities|Casting|CastToLCGameMode (Game|GetGameMode)))
    (Default|RestartLevel _aslcgame_mode)))

(event Input|ActionEvents|InputActionPreviousChampion
  (params (Key :type Key%20Structure))
  ;[1 1 1] Champion selecting
  (:Pressed
    (bind _newchampion (CallFunction|DeterminePreviousChampion))
    (CallFunction|PossesChampion _newchampion)))

(event Input|ActionEvents|InputActionNextChampion
  (params (Key :type Key%20Structure))
  ;[1 1 1] Champion selecting
  (:Pressed
    (bind _newchampion (CallFunction|DetermineNextChampion))
    (CallFunction|PossesChampion _newchampion)))

(event Input|ActionEvents|InputActionZoomIn
  (params (Key :type Key%20Structure))
  ;[1 1 1] Zoom In/Out
  (:Pressed
    (Default|Zoomin (.AsLCPlayer%20Camera (Utilities|Casting|CastToLCPlayerCamera (Variables|Default|GetGameCamera))))))

(event Input|ActionEvents|InputActionZoomOut
  (params (Key :type Key%20Structure))
  ;[1 1 1] Zoom In/Out
  (:Pressed
    (Default|ZoomOut (.AsLCPlayer%20Camera (Utilities|Casting|CastToLCPlayerCamera (Variables|Default|GetGameCamera))))))

(event Input|ActionEvents|InputActionMenu
  (params (Key :type Key%20Structure))
  ;[1 1 1] Menu
  (:Pressed
    (Game|QuitGame 0 "Quit")))

(event Input|AxisEvents|InputAxisLookUp
  (params (AxisValue :type Float%20%28single-precision%29))
  ;[1 1 1] Camera - Mouse
  (Class|PlayerController|AddPitchInput AxisValue))

(event Input|AxisEvents|InputAxisLookRight
  (params (AxisValue :type Float%20%28single-precision%29))
  ;[1 1 1] Camera - Mouse
  (Class|PlayerController|AddYawInput AxisValue))

(event Input|AxisEvents|InputAxisLookUpRate
  (params (AxisValue :type Float%20%28single-precision%29))
  ;[1 1 1] Camera - Controller
  (Class|PlayerController|AddPitchInput (* AxisValue (Variables|Default|GetBaseLookUpRate) (Utilities|Time|GetWorldDeltaSeconds))))

(event Input|AxisEvents|InputAxisLookRightRate
  (params (AxisValue :type Float%20%28single-precision%29))
  ;[1 1 1] Camera - Controller
  (Class|PlayerController|AddYawInput (* AxisValue (Variables|Default|GetBaseLookRightRate) (Utilities|Time|GetWorldDeltaSeconds))))

(fn ConstructionScript
  ;[1 1 1] Timeline
  (Components|Timeline|SetPlayRate (Variables|Default|GetIntroCamTimeline) (Variables|Default|GetIntroCamPlayRate)))

(fn SetChampionReferences
  (params (Warrior :type Character%20Object%20Reference) (Wizard :type Character%20Object%20Reference) (Druid :type Character%20Object%20Reference))
  ;[1 1 1] Init vars
  (Variables|Default|SetWarrior Warrior)
  (Variables|Default|SetWizard Wizard)
  (Variables|Default|SetDruid Druid)
  ;[1 1 1] Champion variables
  (bind _output_get (Variables|Default|SetCharacterList (Utilities|Array|MakeArray (Variables|Default|GetWarrior) (Variables|Default|GetWizard) (Variables|Default|GetDruid))))
  (bind _output_get_2 (Variables|Default|SetCurrentCharacter (Utilities|Array|Get(acopy) _output_get)))
  (CallFunction|PossesChampion _output_get_2)
  ;[1 1 1] Return
  (return true))

(fn DeterminePreviousChampion
  (if (== (Utilities|Array|FindItem (Variables|Default|GetCharacterList) (Variables|Default|GetCurrentCharacter)) 0)
    (LocalVariables|SetNewCharacterLocal (Utilities|Array|Get(acopy) (Variables|Default|GetCharacterList) (- (Utilities|Array|Length (Variables|Default|GetCharacterList)) 1)))
    (else
      (LocalVariables|SetNewCharacterLocal (Utilities|Array|Get(acopy) (Variables|Default|GetCharacterList) (- (Utilities|Array|FindItem (Variables|Default|GetCharacterList) (Variables|Default|GetCurrentCharacter)) 1)))))
  (return (LocalVariables|GetNewCharacterLocal)))

(fn DetermineNextChampion
  (if (== (Utilities|Array|FindItem (Variables|Default|GetCharacterList) (Variables|Default|GetCurrentCharacter)) (- (Utilities|Array|Length (Variables|Default|GetCharacterList)) 1))
    (LocalVariables|SetNewCharacterLocal (Utilities|Array|Get(acopy) (Variables|Default|GetCharacterList)))
    (else
      (LocalVariables|SetNewCharacterLocal (Utilities|Array|Get(acopy) (Variables|Default|GetCharacterList) (+ (Utilities|Array|FindItem (Variables|Default|GetCharacterList) (Variables|Default|GetCurrentCharacter)) 1)))))
  (return (LocalVariables|GetNewCharacterLocal)))

(fn PossesChampion
  (params (NewChampion :type Character%20Object%20Reference))
  ;[1 1 1] Init vars
  (LocalVariables|SetNewChampionLocal NewChampion)
  ;[1 1 1] Store rotation and then detach camera
  (Variables|Default|SetSavedControlRotation (Pawn|GetControlRotation :!class /Script/Engine.Controller))
  (Class|Actor|DetachRootComponentfromParent (Variables|Default|GetGameCamera) true)
  ;[1 1 1] Update new variable and posses new pawn
  (Variables|Default|SetPreviousCharacter (Variables|Default|GetCurrentCharacter))
  (Variables|Default|SetCurrentCharacter (LocalVariables|GetNewChampionLocal))
  (Pawn|Possess (LocalVariables|GetNewChampionLocal))
  ;[1 1 1] Match old control rotation and then play camera animation sequence
  (Pawn|SetControlRotation (Variables|Default|GetSavedControlRotation))
  (Class|Actor|AttachRootComponenttoActor (Variables|Default|GetGameCamera) self "None" "KeepWorldPosition" true)
  (CallFunction|PlayCamtoCharAnimation (LocalVariables|GetNewChampionLocal))
  (Default|CallPossessedNewChampion (LocalVariables|GetNewChampionLocal))
  (return))

(fn CreatePlayerCamera
  ;[1 1 1] Camera
  (bind _returnvalue (Game|SpawnActorfromClass "/Game/Blueprints/Character/LCPlayerCamera.LCPlayerCamera_C" (Math|Transform|MakeTransform (Transformation|GetActorLocation)) "AlwaysSpawn" 0 0))
  (Variables|Default|SetGameCamera _returnvalue)
  (Game|Player|SetViewTargetwithBlend (Variables|Default|GetGameCamera) 0.0 "VTBlend_Linear" 0.0 false)
  (Class|Actor|AttachRootComponenttoActor (Variables|Default|GetGameCamera) self "None" "KeepRelativeOffset" true)
  (return))