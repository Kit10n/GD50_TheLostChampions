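; AI controller for LC characters that runs the possessed LCCharacterBase pawn's own behavior tree and detects player champions.
; Perception updates cast each actor to Druid, Warrior or Wizard and write living ones to a blackboard key named for that class.
; Those champion keys are only set here, never cleared.
; Setter functions expose target, wander, patrol path, death and hit state to the blackboard.
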(event OnPerceptionUpdated(AIPerception)
  (params (UpdatedActors :type Array%20of%20Actor%20Object%20References))
  ;[1 1 1] Sensing the player
  (for _array_element UpdatedActors
    (bind _aslccharacter_druid (Utilities|Casting|CastToLCCharacter_Druid _array_element)
      (:then
        (CallFunction|SetChampionTarget _aslccharacter_druid "Druid"))
      (:CastFailed
        (bind _aslccharacter_warrior (Utilities|Casting|CastToLCCharacter_Warrior _array_element)
          (:then
            (CallFunction|SetChampionTarget _aslccharacter_warrior "Warrior"))
          (:CastFailed
            (bind _aslccharacter_wizard (Utilities|Casting|CastToLCCharacter_Wizard _array_element))
            (CallFunction|SetChampionTarget _aslccharacter_wizard "Wizard")))))))

(event EventOnPossess
  (params (PossessedPawn :type Pawn%20Object%20Reference))
  ;[1 1 1] Run behavior tree
  (AI|RunBehaviorTree (Variables|/Game/Blueprints/Character/LCCharacterBase.LCCharacterBase_C|GetBehaviourTree (.AsLCCharacter%20Base (Utilities|Casting|CastToLCCharacterBase PossessedPawn)))))

(fn ConstructionScript)

(fn SetTarget
  (params (NewAITarget :type Actor%20Object%20Reference))
  (AI|Components|Blackboard|SetValueasObject (AI|GetBlackboard self) (Utilities|Name|MakeLiteralName "Target") NewAITarget))

(fn SetChampionTarget
  (params (Champion :type LC%20Character%20Base%20Object%20Reference) (KeyName :type Name))
  (if (not (Variables|/Game/Blueprints/Character/LCCharacterBase.LCCharacterBase_C|GetIsDead Champion))
    (AI|Components|Blackboard|SetValueasObject (AI|GetBlackboard self) KeyName Champion)))

(fn SetWander
  (params (Wander :type Boolean))
  (AI|Components|Blackboard|SetValueasBool (AI|GetBlackboard self) (Utilities|Name|MakeLiteralName "Wander") Wander))

(fn SetPatrolPath
  (params (PatrolPath :type LC%20Patrol%20Path%20Object%20Reference))
  (AI|Components|Blackboard|SetValueasObject (AI|GetBlackboard self) (Utilities|Name|MakeLiteralName "PatrolPath") PatrolPath))

(fn SetIsDead
  (params (IsDead :type Boolean))
  (AI|Components|Blackboard|SetValueasBool (AI|GetBlackboard self) (Utilities|Name|MakeLiteralName "IsDead") IsDead))

(fn SetIsHit
  (params (IsHit :type Boolean))
  (AI|Components|Blackboard|SetValueasBool (AI|GetBlackboard self) (Utilities|Name|MakeLiteralName "IsHit") IsHit))