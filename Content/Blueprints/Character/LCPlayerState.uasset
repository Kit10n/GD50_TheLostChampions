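; Player state Blueprint that tracks the player's collected coins and gems.
; AddCoins adds a given amount to Coins and AddGem increments Gems by one.
; Each function then calls its gain event, GainedCoin or GainedGem, and returns true.
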(fn ConstructionScript)

(fn AddCoins
  (params (Amount :type Integer))
  ;[1 1 1] Coins!
  (Variables|Default|SetCoins (+ Amount (Variables|Default|GetCoins)))
  (Default|CallGainedCoin)
  (return true))

(fn AddGem
  ;[1 1 1] Gems!
  (Variables|Default|SetGems (+ (Variables|Default|GetGems) 1))
  (Default|CallGainedGem)
  (return true))