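; LCSquidInk is a squid ink projectile that deals damage to whatever it strikes.
; Hit and overlap events on its collision component both ignore the owner and other ink projectiles through two check macros.
; On landing it stops movement, applies damage credited to its instigator's controller, disables collision, spawns an explosion particle effect and destroys itself.
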(event OnComponentHit(InkCollision)
  (params (OtherActor :type Actor%20Object%20Reference) (OtherComp :type Primitive%20Component%20Object%20Reference) (NormalImpulse :type Vector :default "0, 0, 0") (Hit :type Hit%20Result%20Structure%20%28by%20ref%29))
  (Utilities|CheckActorIsOwner OtherActor
    (:False
      (Utilities|CheckActorIsSameClass OtherActor
        (:False
          (CallFunction|ProjectileLanded OtherActor OtherComp))))))

(event OnComponentBeginOverlap(InkCollision)
  (params (OtherActor :type Actor%20Object%20Reference) (OtherComp :type Primitive%20Component%20Object%20Reference) (OtherBodyIndex :type Integer) (bFromSweep :type Boolean) (SweepResult :type Hit%20Result%20Structure%20%28by%20ref%29))
  (Utilities|CheckActorIsOwner OtherActor
    (:False
      (Utilities|CheckActorIsSameClass OtherActor
        (:False
          (CallFunction|ProjectileLanded OtherActor OtherComp))))))

(fn ConstructionScript)

(fn ProjectileLanded
  (params (HitActor :type Actor%20Object%20Reference) (HitComponent :type Scene%20Component%20Object%20Reference))
  ;[1 1 1] Init
  (LocalVariables|SetHitCharacterLocal HitActor)
  (LocalVariables|SetHitComponentLocal HitComponent)
  ;[1 1 1] Stop the movement
  (Components|Movement|StopMovementImmediately (Variables|Default|GetProjectileMovement))
  (Utilities|IsValid (LocalVariables|GetHitCharacterLocal)
    (:Is%20Valid
      (Game|Damage|ApplyDamage (LocalVariables|GetHitCharacterLocal) (Variables|Default|GetDamage) (Game|GetInstigatorController) self))
    (:Is%20Not%20Valid
      _))
  (Collision|SetCollisionEnabled (Variables|Default|GetInkCollision) "NoCollision")
  (Effects|SpawnEmitteratLocation "/Game/Effects/Particles/Systems/PS_SquidInkExplosion.PS_SquidInkExplosion" (Transformation|GetActorLocation) (Transformation|GetActorRotation))
  (Actor|DestroyActor))