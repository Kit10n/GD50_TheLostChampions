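; Player camera Blueprint that provides animated zoom in and out by changing the spring arm's length.
; ZoomIn and ZoomOut trigger events that step the target length by ZoomAmount, clamp it to min/max limits, and restart a shared timeline.
; The timeline lerps from the current length toward the target on each update, compounding the easing.
; The construction script sets the timeline's speed from ZoomPlayRate.
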(event Custom|PlayZoomInAnimation
  ;[1 1 1] Zoom in and out animation
  (Variables|Default|SetNewTargetArmLength (Math|Float|Clamp(Float) (- (Variables|/Script/Engine.SpringArmComponent|GetTargetArmLength (Variables|Default|GetSpringArm)) (Variables|Default|GetZoomAmount)) (Variables|Default|GetMinTargetArmLength) (Variables|Default|GetMaxTargetArmLength)))
  (bind _0_1 (Timeline|ZoomTimeline PlayFromStart)
    (:Update
      (Variables|/Script/Engine.SpringArmComponent|SetTargetArmLength (Variables|Default|GetSpringArm) (Math|Float|Lerp (Variables|/Script/Engine.SpringArmComponent|GetTargetArmLength (Variables|Default|GetSpringArm)) (Variables|Default|GetNewTargetArmLength) _0_1)))))

(event Custom|PlayZoomOutAnimation
  ;[1 1 1] Zoom in and out animation
  (Variables|Default|SetNewTargetArmLength (Math|Float|Clamp(Float) (+ (Variables|/Script/Engine.SpringArmComponent|GetTargetArmLength (Variables|Default|GetSpringArm)) (Variables|Default|GetZoomAmount)) (Variables|Default|GetMinTargetArmLength) (Variables|Default|GetMaxTargetArmLength)))
  (bind _0_1 (Timeline|ZoomTimeline PlayFromStart)
    (:Update
      (Variables|/Script/Engine.SpringArmComponent|SetTargetArmLength (Variables|Default|GetSpringArm) (Math|Float|Lerp (Variables|/Script/Engine.SpringArmComponent|GetTargetArmLength (Variables|Default|GetSpringArm)) (Variables|Default|GetNewTargetArmLength) _0_1)))))

(fn ConstructionScript
  (Components|Timeline|SetPlayRate (Variables|Default|GetZoomTimeline) (Variables|Default|GetZoomPlayRate)))

(fn Zoomin
  (CallFunction|PlayZoominAnimation))

(fn ZoomOut
  (CallFunction|PlayZoomOutAnimation))