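; Wizard character Blueprint that can conjure a protective barrier, cycling it between no barrier, front and top positions.
; Each CreateBarrier call destroys the current barrier, advances the cycle index, and spawns any new LCWizardBarrier attached to that position's arrow component.
; The front barrier disables orient-rotation-to-movement, while the other states re-enable it.
; The death sequence override destroys any active barrier before calling the parent.
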(event EventPlayDeathSequenceAnimaiton
  (Utilities|IsValid (Variables|Default|GetCurrentBarrier)
    (:Is%20Valid
      (Actor|DestroyActor (Variables|Default|GetCurrentBarrier)))
    (:Is%20Not%20Valid
      _))
  (|CallParentFunction))

(fn ConstructionScript
  (|CallParentFunction))

(fn CreateBarrier
  ;[1 1 1] Remove any previous barriers
  (Utilities|IsValid (Variables|Default|GetCurrentBarrier)
    (:Is%20Valid
      (Actor|DestroyActor (Variables|Default|GetCurrentBarrier)))
    (:Is%20Not%20Valid
      _))
  ;[1 1 1] Which are we on?
  (switch int (Variables|Default|GetBarrierCycleIndex)
    (:Default
      (Variables|Default|SetBarrierCycleIndex 1 :!label _label)
      (Variables|/Script/Engine.CharacterMovementComponent|SetbOrientRotationToMovement (Variables|Character|GetCharacterMovement) true))
    (:0
      (goto _label))
    (:1
      (LocalVariables|SetBarrierSpawnLocal (Variables|Default|GetFrontBarrierArrow))
      (Variables|Default|SetBarrierCycleIndex 2)
      (Variables|/Script/Engine.CharacterMovementComponent|SetbOrientRotationToMovement (Variables|Character|GetCharacterMovement) false)
      ;[1 1 1] Spawn and attach the barrier
      (bind _returnvalue (Game|SpawnActorfromClass "/Game/Blueprints/Character/LCWizardBarrier.LCWizardBarrier_C" (Transformation|GetWorldTransform (LocalVariables|GetBarrierSpawnLocal)) "AlwaysSpawn" 0 0 :!label _label_2))
      (bind _output_get (Variables|Default|SetCurrentBarrier _returnvalue))
      (Class|Actor|AttachRootComponentto _output_get (LocalVariables|GetBarrierSpawnLocal) "None" "SnapToTarget" true))
    (:2
      (LocalVariables|SetBarrierSpawnLocal (Variables|Default|GetTopBarrierArrow))
      (Variables|Default|SetBarrierCycleIndex 0)
      (Variables|/Script/Engine.CharacterMovementComponent|SetbOrientRotationToMovement (Variables|Character|GetCharacterMovement) true)
      (goto _label_2))))