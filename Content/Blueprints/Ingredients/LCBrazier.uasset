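; LCBrazier is a dungeon brazier ingredient that can be lit or unlit.
; SetBrazierLit stores the IsLit state, toggles the light and fire particle, and swaps between lit and unlit firepit meshes.
; It calls the OnBrazierLit dispatcher on every update, including when unlit.
; Both the construction script and BeginPlay apply IsLit, so the placed brazier reflects its setting before play and at startup.
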(event EventBeginPlay
  (CallFunction|SetBrazierLit (Variables|Brazier|GetIsLit)))

(fn ConstructionScript
  (CallFunction|SetBrazierLit (Variables|Brazier|GetIsLit)))

(fn SetBrazierLit
  (params (IsLit :type Boolean))
  (bind _brazierfireparticle (Variables|Default|GetBrazierFireParticle))
  (bind _output_get (LocalVariables|SetIsLitLocal IsLit))
  (Variables|Brazier|SetIsLit _output_get)
  (Rendering|SetVisibility (Variables|Default|GetBrazierLight) (LocalVariables|GetIsLitLocal) false)
  (if (LocalVariables|GetIsLitLocal)
    (Components|Activation|Activate _brazierfireparticle false)
    (else
      (Components|Activation|Deactivate _brazierfireparticle)))
  (Components|StaticMesh|SetStaticMesh (Variables|Default|GetBrazierMesh) (select (LocalVariables|GetIsLitLocal) "/Game/Props/Dungeon/Meshes/PropDungeon_FirepitLarge_Lit.PropDungeon_FirepitLarge_Lit" "/Game/Props/Dungeon/Meshes/PropDungeon_FirepitLarge_Unlit.PropDungeon_FirepitLarge_Unlit"))
  (Default|CallOnBrazierLit self))