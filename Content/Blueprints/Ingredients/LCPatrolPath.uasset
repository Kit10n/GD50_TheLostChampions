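; LCPatrolPath is a spline-based patrol path actor that holds a wait time for each point.
; The construction script sizes the wait-time array to the spline's point count and spawns a numbered, unattached text label just above each point.
; On BeginPlay, the debug-draw flag either unhides the spline in game or hides the labels.
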(event EventBeginPlay
  ;[1 1 1] Hide and show stuff based on Debug Draw In Game bool
  (if (Variables|PatrolPath|GetDebugDrawInGame)
    (Development|SetHiddeninGame (Variables|Default|GetSpline) false false)
    (else
      (for _array_element (Variables|PatrolPath|GetTextRenderers)
        (bind _astext_render_component (Utilities|Casting|CastToTextRenderComponent _array_element))
        (Rendering|SetVisibility _astext_render_component false false)))))

(fn ConstructionScript
  ;[1 1 1] Time to wait at each point
  (Utilities|Array|Resize (Variables|PatrolPath|GetPointWaitTime) (Spline|GetNumberOfSplinePoints (Variables|Default|GetSpline)))
  ;[1 1 1] Text rendering based off number of points
  (Utilities|Array|Clear (Variables|PatrolPath|GetTextRenderers))
  (for _index (range 0 (- (Spline|GetNumberOfSplinePoints (Variables|Default|GetSpline)) 1))
    (bind _returnvalue (AddComponent|AddTextRenderComponent true (Math|Transform|MakeTransform (+ (Spline|GetLocationatSplinePoint (Variables|Default|GetSpline) _index "World") "0, 0,25.000000") (Transformation|GetWorldRotation (Variables|Default|GetSpline)) "1,1,1")))
    (Utilities|Array|Add (Variables|PatrolPath|GetTextRenderers) _returnvalue)
    (Rendering|Components|TextRender|SetText _returnvalue (Utilities|Text|ToText(Integer) _index))
    (Rendering|Components|TextRender|SetTextRenderColor _returnvalue (Math|Conversions|ToColor(LinearColor) (Variables|PatrolPath|GetTextColour)))
    (Rendering|Components|TextRender|SetWorldSize _returnvalue (Variables|PatrolPath|GetTextSize))))