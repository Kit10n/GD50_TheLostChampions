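; Rotating platform that turns in 90-degree steps, clockwise or counterclockwise, on request or automatically.
; One timeline drives both directions, played forward or in reverse, with its play rate set from MoveTime in the construction script.
; Each finished turn fires a notification; auto-rotate then waits StopTime and continues in a circular loop or ping-pong.
; Requests during movement store only the latest direction, replayed afterward when auto-rotate is off.
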(event Custom|RotatePlatformClockwise
  ;[1 1 1] Events
  ;[1 1 1] Queue or move
  (if (not (Variables|Platform|GetIsMoving))
    (Variables|Platform|SetStartRotation (Transformation|GetWorldRotation (Variables|Default|GetPlatformRoot)))
    ;[1 1 1] Rotation
    (bind (_direction _0_1) (Timeline|RotatingPlatformTimeline PlayFromStart)
      (:Update
        (Variables|Platform|SetIsMoving true)
        (Variables|Platform|SetCurrentDirection _direction)
        (Transformation|SetRelativeRotation (Variables|Default|GetPlatformRoot) (Math|Rotator|Lerp(Rotator) (Utilities|Select :Index (Variables|Platform|GetCurrentDirection) :Forward (Variables|Platform|GetStartRotation) :Backward (Math|Rotator|CombineRotators (Variables|Platform|GetStartRotation) (Utilities|Select :Index (Variables|Platform|GetCurrentDirection) :Forward "0,90.000000,0" :Backward "0,-90.000000,0"))) (Utilities|Select :Index (Variables|Platform|GetCurrentDirection) :Forward (Math|Rotator|CombineRotators (Variables|Platform|GetStartRotation) (Utilities|Select :Index (Variables|Platform|GetCurrentDirection) :Forward "0,90.000000,0" :Backward "0,-90.000000,0")) :Backward (Variables|Platform|GetStartRotation)) _0_1 true) false false))
      (:Finished
        (Variables|Platform|SetIsMoving false)
        (Variables|Platform|SetCurrentDirection _direction)
        ;[1 1 1] Event
        (Default|CallOnPlatformFinishedMoving self (Variables|Platform|GetCurrentDirection))
        ;[1 1 1] Auto play system
        (if (Variables|Platform|GetAutoRotate)
          (Utilities|FlowControl|Delay (Variables|Platform|GetStopTime))
          (switch Utilities|FlowControl|Switch|SwitchonEnum_RotatingMovementType (Variables|Platform|GetAutoRotateMovementType)
            (:NewEnumerator1
              (switch Utilities|FlowControl|Switch|SwitchonETimelineDirection (Variables|Platform|GetCurrentDirection)
                (:Forward
                  (CallFunction|RotatePlatformClockwise))
                (:Backward
                  (CallFunction|RotatePlatformCounterclockwise))))
            (:NewEnumerator0
              (switch Utilities|FlowControl|Switch|SwitchonETimelineDirection (Variables|Platform|GetCurrentDirection)
                (:Forward
                  (CallFunction|RotatePlatformCounterclockwise))
                (:Backward
                  (CallFunction|RotatePlatformClockwise)))))
          (else
            ;[1 1 1] Queue system
            (if (Variables|Platform|GetIsMoveQueued)
              (Variables|Platform|SetIsMoveQueued false)
              (switch Utilities|FlowControl|Switch|SwitchonETimelineDirection (Variables|Platform|GetQueuedMove)
                (:Forward
                  (CallFunction|RotatePlatformClockwise))
                (:Backward
                  (CallFunction|RotatePlatformCounterclockwise))))))))
    (else
      (Variables|Platform|SetIsMoveQueued true)
      (Variables|Platform|SetQueuedMove "Forward"))))

(event Custom|RotatePlatformCounterclockwise
  ;[1 1 1] Events
  ;[1 1 1] Queue or move
  (if (not (Variables|Platform|GetIsMoving))
    (Variables|Platform|SetStartRotation (Transformation|GetWorldRotation (Variables|Default|GetPlatformRoot)))
    ;[1 1 1] Rotation
    (bind (_direction _0_1) (Timeline|RotatingPlatformTimeline ReverseFromEnd)
      (:Update
        (Variables|Platform|SetIsMoving true)
        (Variables|Platform|SetCurrentDirection _direction)
        (Transformation|SetRelativeRotation (Variables|Default|GetPlatformRoot) (Math|Rotator|Lerp(Rotator) (Utilities|Select :Index (Variables|Platform|GetCurrentDirection) :Forward (Variables|Platform|GetStartRotation) :Backward (Math|Rotator|CombineRotators (Variables|Platform|GetStartRotation) (Utilities|Select :Index (Variables|Platform|GetCurrentDirection) :Forward "0,90.000000,0" :Backward "0,-90.000000,0"))) (Utilities|Select :Index (Variables|Platform|GetCurrentDirection) :Forward (Math|Rotator|CombineRotators (Variables|Platform|GetStartRotation) (Utilities|Select :Index (Variables|Platform|GetCurrentDirection) :Forward "0,90.000000,0" :Backward "0,-90.000000,0")) :Backward (Variables|Platform|GetStartRotation)) _0_1 true) false false))
      (:Finished
        (Variables|Platform|SetIsMoving false)
        (Variables|Platform|SetCurrentDirection _direction)
        ;[1 1 1] Event
        (Default|CallOnPlatformFinishedMoving self (Variables|Platform|GetCurrentDirection))
        ;[1 1 1] Auto play system
        (if (Variables|Platform|GetAutoRotate)
          (Utilities|FlowControl|Delay (Variables|Platform|GetStopTime))
          (switch Utilities|FlowControl|Switch|SwitchonEnum_RotatingMovementType (Variables|Platform|GetAutoRotateMovementType)
            (:NewEnumerator1
              (switch Utilities|FlowControl|Switch|SwitchonETimelineDirection (Variables|Platform|GetCurrentDirection)
                (:Forward
                  (CallFunction|RotatePlatformClockwise))
                (:Backward
                  (CallFunction|RotatePlatformCounterclockwise))))
            (:NewEnumerator0
              (switch Utilities|FlowControl|Switch|SwitchonETimelineDirection (Variables|Platform|GetCurrentDirection)
                (:Forward
                  (CallFunction|RotatePlatformCounterclockwise))
                (:Backward
                  (CallFunction|RotatePlatformClockwise)))))
          (else
            ;[1 1 1] Queue system
            (if (Variables|Platform|GetIsMoveQueued)
              (Variables|Platform|SetIsMoveQueued false)
              (switch Utilities|FlowControl|Switch|SwitchonETimelineDirection (Variables|Platform|GetQueuedMove)
                (:Forward
                  (CallFunction|RotatePlatformClockwise))
                (:Backward
                  (CallFunction|RotatePlatformCounterclockwise))))))))
    (else
      (Variables|Platform|SetIsMoveQueued true)
      (Variables|Platform|SetQueuedMove "Backward"))))

(event EventBeginPlay
  ;[1 1 1] Auto play the rotation if it's set so
  (if (Variables|Platform|GetAutoRotate)
    (switch Utilities|FlowControl|Switch|SwitchonEnum_CircularMotion (Variables|Platform|GetAutoRotateInitialDirection)
      (:NewEnumerator0
        (CallFunction|RotatePlatformClockwise))
      (:NewEnumerator1
        (CallFunction|RotatePlatformCounterclockwise)))))

(fn ConstructionScript
  ;[1 1 1] Set length of timeline
  (Components|Timeline|SetPlayRate (Variables|Default|GetRotatingPlatformTimeline) (/ 1.0 (Variables|Platform|GetMoveTime))))

(fn SetAutoRotate
  (params (AutoRotate :type Boolean))
  (Variables|Platform|SetAutoRotate AutoRotate))