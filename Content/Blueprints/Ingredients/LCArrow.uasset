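; LCArrow is an arrow projectile that damages what it strikes and sticks into it.
; Collision hits and overlaps, ignoring its owner and other arrows of its class, call ProjectileLanded, which stops movement and applies damage.
; It then attaches at world position (using a Character's mesh, socket HeadSocket) and disables collision.
; A timeline wobbles the tip with adjustable intensity and rate, then the arrow destroys itself after a short delay.
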(event OnComponentHit(ArrowCollision)
  (params (OtherActor :type Actor%20Object%20Reference) (OtherComp :type Primitive%20Component%20Object%20Reference) (NormalImpulse :type Vector :default "0, 0, 0") (Hit :type Hit%20Result%20Structure%20%28by%20ref%29))
  ;[1 1 1] Hit and overlap events
  (Utilities|CheckActorIsOwner OtherActor
    (:False
      (Utilities|CheckActorIsArrow OtherActor
        (:false
          (CallFunction|ProjectileLanded OtherActor OtherComp))))))

(event OnComponentBeginOverlap(ArrowCollision)
  (params (OtherActor :type Actor%20Object%20Reference) (OtherComp :type Primitive%20Component%20Object%20Reference) (OtherBodyIndex :type Integer) (bFromSweep :type Boolean) (SweepResult :type Hit%20Result%20Structure%20%28by%20ref%29))
  ;[1 1 1] Hit and overlap events
  (Utilities|CheckActorIsOwner OtherActor
    (:False
      (Utilities|CheckActorIsArrow OtherActor
        (:false
          (CallFunction|ProjectileLanded OtherActor OtherComp))))))

(event Custom|PlayBoingAnimation
  (bind _boingintensity (Variables|Default|GetBoingIntensity))
  ;[1 1 1] Boing animation
  (bind _rotating (Timeline|BoingTimeline Play)
    (:Update
      (Transformation|SetRelativeRotation (Variables|Default|GetArrowTipScene) (Class|KismetMathLibrary|MakeRot (* (.X (Math|Vector|BreakVector _rotating)) _boingintensity) (* (.Y (Math|Vector|BreakVector _rotating)) _boingintensity) 0.0) false))
    (:Finished
      (Utilities|FlowControl|Delay 1.0)
      (Actor|DestroyActor))))

(fn ConstructionScript
  ;[1 1 1] Timeline
  (Components|Timeline|SetPlayRate (Variables|Default|GetBoingTimeline) (Variables|Default|GetBoingPlayRate)))

(fn ProjectileLanded
  (params (HitCharacter :type Actor%20Object%20Reference) (HitComponent :type Scene%20Component%20Object%20Reference))
  ;[1 1 1] Init
  (LocalVariables|SetHitActorLocal HitCharacter)
  (LocalVariables|SetHitComponentLocal HitComponent)
  ;[1 1 1] Stop! Hammer time
  (Components|Movement|StopMovementImmediately (Variables|Default|GetArrowMovement))
  ;[1 1 1] Did we hit something valid?
  (Utilities|IsValid (LocalVariables|GetHitActorLocal)
    (:Is%20Valid
      ;[1 1 1] Damage them, check if they are a character
      (Game|Damage|ApplyDamage (LocalVariables|GetHitActorLocal) (Variables|Default|GetArrowDamage) 0 0)
      (bind _ascharacter (Utilities|Casting|CastToCharacter (LocalVariables|GetHitActorLocal))
        (:then
          (LocalVariables|SetHitComponentLocal (Variables|/Script/Engine.Character|GetMesh _ascharacter)))
        (:CastFailed
          _)))
    (:Is%20Not%20Valid
      _))
  ;[1 1 1] Attach to what we hit, play the boing animation and turn off collision
  (Class|Actor|AttachRootComponentto (LocalVariables|GetHitComponentLocal) "HeadSocket" "KeepWorldPosition" true)
  (CallFunction|PlayBoingAnimation)
  (Collision|SetCollisionEnabled (Variables|Default|GetArrowCollision) "NoCollision"))