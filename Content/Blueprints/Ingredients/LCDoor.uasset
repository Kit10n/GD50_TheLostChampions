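; LCDoor is a configurable double dungeon door with wood, stone, steel or epic meshes and an optional archway.
; The construction script applies meshes and open speed, while BeginPlay snaps doors flagged open by default to open.
; Open, close and toggle events drive one timeline forward or backward, mirroring both hinges' yaw and firing opened or closed notifications when finished.
; A locked-door shake animation exists but is unconnected, and no lock check is implemented.
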(event Custom|OpenDoor
  ;[1 1 1] Open/close the door only if it's unlocked
  (Variables|Door|SetPlayerInteracted false)
  ;[1 1 1] Animation timeline: Rotate the doors
  (bind (_direction _0_1) (Timeline|OpenDoorTimeline Play)
    (:Update
      (Transformation|SetRelativeRotation (Variables|Default|GetDoorRightHinge) (Math|Rotator|MakeRotator 0.0 0.0 (Math|Float|Lerp 0.0 (Variables|Door|GetDoorOpenAngle) _0_1)) false false)
      (Transformation|SetRelativeRotation (Variables|Default|GetDoorLeftHinge) (Math|Rotator|MakeRotator 0.0 0.0 (Math|Float|Lerp 0.0 (* (Variables|Door|GetDoorOpenAngle) -1.0) _0_1)) false false))
    (:Finished
      ;[1 1 1] Set door open state
      (switch Utilities|FlowControl|Switch|SwitchonETimelineDirection _direction
        (:Forward
          (Variables|Door|SetDoorIsOpen true)
          ;[1 1 1] Let the world know we opened/closed
          (Default|CallOnDoorOpened (Variables|Door|GetPlayerInteracted)))
        (:Backward
          (Variables|Door|SetDoorIsOpen false)
          (Default|CallOnDoorClosed (Variables|Door|GetPlayerInteracted)))))))

(event Custom|CloseDoor
  ;[1 1 1] Open/close the door only if it's unlocked
  (Variables|Door|SetPlayerInteracted false)
  ;[1 1 1] Animation timeline: Rotate the doors
  (bind (_direction _0_1) (Timeline|OpenDoorTimeline Reverse)
    (:Update
      (Transformation|SetRelativeRotation (Variables|Default|GetDoorRightHinge) (Math|Rotator|MakeRotator 0.0 0.0 (Math|Float|Lerp 0.0 (Variables|Door|GetDoorOpenAngle) _0_1)) false false)
      (Transformation|SetRelativeRotation (Variables|Default|GetDoorLeftHinge) (Math|Rotator|MakeRotator 0.0 0.0 (Math|Float|Lerp 0.0 (* (Variables|Door|GetDoorOpenAngle) -1.0) _0_1)) false false))
    (:Finished
      ;[1 1 1] Set door open state
      (switch Utilities|FlowControl|Switch|SwitchonETimelineDirection _direction
        (:Forward
          (Variables|Door|SetDoorIsOpen true)
          ;[1 1 1] Let the world know we opened/closed
          (Default|CallOnDoorOpened (Variables|Door|GetPlayerInteracted)))
        (:Backward
          (Variables|Door|SetDoorIsOpen false)
          (Default|CallOnDoorClosed (Variables|Door|GetPlayerInteracted)))))))

(event Custom|ToggleDoorOpen
  ;[1 1 1] Open/close the door only if it's unlocked
  (Variables|Door|SetPlayerInteracted false)
  (if (not (Variables|Door|GetDoorIsOpen))
    ;[1 1 1] Animation timeline: Rotate the doors
    (bind (_direction _0_1) (Timeline|OpenDoorTimeline Play)
      (:Update
        (Transformation|SetRelativeRotation (Variables|Default|GetDoorRightHinge) (Math|Rotator|MakeRotator 0.0 0.0 (Math|Float|Lerp 0.0 (Variables|Door|GetDoorOpenAngle) _0_1)) false false)
        (Transformation|SetRelativeRotation (Variables|Default|GetDoorLeftHinge) (Math|Rotator|MakeRotator 0.0 0.0 (Math|Float|Lerp 0.0 (* (Variables|Door|GetDoorOpenAngle) -1.0) _0_1)) false false))
      (:Finished
        ;[1 1 1] Set door open state
        (switch Utilities|FlowControl|Switch|SwitchonETimelineDirection _direction
          (:Forward
            (Variables|Door|SetDoorIsOpen true)
            ;[1 1 1] Let the world know we opened/closed
            (Default|CallOnDoorOpened (Variables|Door|GetPlayerInteracted)))
          (:Backward
            (Variables|Door|SetDoorIsOpen false)
            (Default|CallOnDoorClosed (Variables|Door|GetPlayerInteracted))))))
    (else
      (Timeline|OpenDoorTimeline Reverse))))

(event EventBeginPlay
  ;[1 1 1] Check if the door is open by default
  (if (Variables|Door|GetOpenByDefault)
    (Components|Timeline|SetPlaybackPosition (Variables|Default|GetOpenDoorTimeline) 1.0 true true)))

(fn ConstructionScript
  ;[1 1 1] Set how fast the door will open
  (Components|Timeline|SetPlayRate (Variables|Default|GetOpenDoorTimeline) (Variables|Door|GetDoorOpenPlayRate))
  ;[1 1 1] Set the door type
  (Door|SetDoorType (Variables|Door|GetDoorType))
  ;[1 1 1] Add the archway mesh
  (if (Variables|Door|GetIncludeArchwayMesh)
    (Components|StaticMesh|SetStaticMesh (Variables|Default|GetArchway) "/Game/Environment/Dungeon/Meshes/Dungeon_Arch01.Dungeon_Arch01")
    ;[1 1 1] If the door is open or not
    (Variables|Door|SetDoorIsOpen (Variables|Door|GetOpenByDefault))))

(fn SetDoorType
  (params (NewDoorType :type Enum_DungeonDoorType%20Enum :default "NewEnumerator0"))
  ;[1 1 1] Init vars
  (LocalVariables|SetNewDoorTypeLocal NewDoorType)
  ;[1 1 1] Set the meshes based off the door type
  (Components|StaticMesh|SetStaticMesh (Variables|Default|GetDoorFrame) (Utilities|Select :Index (LocalVariables|GetNewDoorTypeLocal) :NewEnumerator0 "/Game/Environment/Dungeon/Meshes/Dungeon_Door_Wood_Frame.Dungeon_Door_Wood_Frame" :NewEnumerator1 "/Game/Environment/Dungeon/Meshes/Dungeon_Door_Stone_Frame.Dungeon_Door_Stone_Frame" :NewEnumerator2 "/Game/Environment/Dungeon/Meshes/Dungeon_Door_Steel_Frame.Dungeon_Door_Steel_Frame" :NewEnumerator3 "/Game/Environment/Dungeon/Meshes/Dungeon_Door_Epic_Frame.Dungeon_Door_Epic_Frame"))
  (Components|StaticMesh|SetStaticMesh (Variables|Default|GetDoorLeft) (Utilities|Select :Index (LocalVariables|GetNewDoorTypeLocal) :NewEnumerator0 "/Game/Environment/Dungeon/Meshes/Dungeon_Door_Wood_Left3.Dungeon_Door_Wood_Left3" :NewEnumerator1 "/Game/Environment/Dungeon/Meshes/Dungeon_Door_Stone_Left.Dungeon_Door_Stone_Left" :NewEnumerator2 "/Game/Environment/Dungeon/Meshes/Dungeon_Door_Steel_Left.Dungeon_Door_Steel_Left" :NewEnumerator3 "/Game/Environment/Dungeon/Meshes/Dungeon_Door_Epic_Left.Dungeon_Door_Epic_Left"))
  (Components|StaticMesh|SetStaticMesh (Variables|Default|GetDoorRight) (Utilities|Select :Index (LocalVariables|GetNewDoorTypeLocal) :NewEnumerator0 "/Game/Environment/Dungeon/Meshes/Dungeon_Door_Wood_Right3.Dungeon_Door_Wood_Right3" :NewEnumerator1 "/Game/Environment/Dungeon/Meshes/Dungeon_Door_Stone_Right.Dungeon_Door_Stone_Right" :NewEnumerator2 "/Game/Environment/Dungeon/Meshes/Dungeon_Door_Steel_Right.Dungeon_Door_Steel_Right" :NewEnumerator3 "/Game/Environment/Dungeon/Meshes/Dungeon_Door_Epic_Right.Dungeon_Door_Epic_Right"))
  ;[1 1 1] Return
  (return))

(fn GetDoorIsOpen
  (return (Variables|Door|GetDoorIsOpen)))