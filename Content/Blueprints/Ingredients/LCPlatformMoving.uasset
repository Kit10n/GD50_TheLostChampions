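; Moving platform that travels between its placed transform and a Destination offset relative to it.
; The construction script caches the start transform, sets the timeline rate from MoveTime and places a preview mesh at the destination.
; A timeline interpolates location and rotation, exposed through play, reverse and toggle events, and broadcasts the direction when finished.
; With AutoPlay, it starts on BeginPlay and shuttles back and forth, pausing for StopTime at each end.
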(event Custom|PlayPlatformMove
  (bind _starttransform (Variables|Platform|GetStartTransform))
  (bind _starttransform_2 (Variables|Platform|GetStartTransform))
  ;[1 1 1] Movement
  (bind (_direction _0_1) (Timeline|PlatformMovementTimeLine Play)
    (:Update
      (Transformation|SetWorldLocationAndRotation (Variables|Default|GetPlatformRoot) (Math|Vector|Lerp(Vector) (.location _starttransform) (+ (.location _starttransform) (Math|Vector|RotateVector (.location (Variables|Platform|GetDestination)) (.rotation (Variables|Platform|GetStartTransform)))) _0_1) (Math|Rotator|Lerp(Rotator) (.rotation _starttransform_2) (Math|Rotator|CombineRotators (.rotation _starttransform_2) (.rotation (Variables|Platform|GetDestination))) _0_1 true) false false))
    (:Finished
      ;[1 1 1] Comment
      (Variables|Platform|SetPlatformMoved (Utilities|Select :Index _direction :Forward true :Backward false))
      (Default|CallOnPlatformFinishedMoving _direction)
      (if (Variables|Platform|GetAutoPlay)
        (Utilities|FlowControl|Delay (Variables|Platform|GetStopTime))
        (switch Utilities|FlowControl|Switch|SwitchonETimelineDirection _direction
          (:Forward
            (CallFunction|ReversePlatformMove))
          (:Backward
            (CallFunction|PlayPlatformMove)))))))

(event Custom|ReversePlatformMove
  (bind _starttransform (Variables|Platform|GetStartTransform))
  (bind _starttransform_2 (Variables|Platform|GetStartTransform))
  ;[1 1 1] Movement
  (bind (_direction _0_1) (Timeline|PlatformMovementTimeLine Reverse)
    (:Update
      (Transformation|SetWorldLocationAndRotation (Variables|Default|GetPlatformRoot) (Math|Vector|Lerp(Vector) (.location _starttransform) (+ (.location _starttransform) (Math|Vector|RotateVector (.location (Variables|Platform|GetDestination)) (.rotation (Variables|Platform|GetStartTransform)))) _0_1) (Math|Rotator|Lerp(Rotator) (.rotation _starttransform_2) (Math|Rotator|CombineRotators (.rotation _starttransform_2) (.rotation (Variables|Platform|GetDestination))) _0_1 true) false false))
    (:Finished
      ;[1 1 1] Comment
      (Variables|Platform|SetPlatformMoved (Utilities|Select :Index _direction :Forward true :Backward false))
      (Default|CallOnPlatformFinishedMoving _direction)
      (if (Variables|Platform|GetAutoPlay)
        (Utilities|FlowControl|Delay (Variables|Platform|GetStopTime))
        (switch Utilities|FlowControl|Switch|SwitchonETimelineDirection _direction
          (:Forward
            (CallFunction|ReversePlatformMove))
          (:Backward
            (CallFunction|PlayPlatformMove)))))))

(event Custom|TogglePlatformMove
  (bind _starttransform (Variables|Platform|GetStartTransform))
  (bind _starttransform_2 (Variables|Platform|GetStartTransform))
  ;[1 1 1] Movement
  (if (not (Variables|Platform|GetPlatformMoved))
    (bind (_direction _0_1) (Timeline|PlatformMovementTimeLine Play)
      (:Update
        (Transformation|SetWorldLocationAndRotation (Variables|Default|GetPlatformRoot) (Math|Vector|Lerp(Vector) (.location _starttransform) (+ (.location _starttransform) (Math|Vector|RotateVector (.location (Variables|Platform|GetDestination)) (.rotation (Variables|Platform|GetStartTransform)))) _0_1) (Math|Rotator|Lerp(Rotator) (.rotation _starttransform_2) (Math|Rotator|CombineRotators (.rotation _starttransform_2) (.rotation (Variables|Platform|GetDestination))) _0_1 true) false false))
      (:Finished
        ;[1 1 1] Comment
        (Variables|Platform|SetPlatformMoved (Utilities|Select :Index _direction :Forward true :Backward false))
        (Default|CallOnPlatformFinishedMoving _direction)
        (if (Variables|Platform|GetAutoPlay)
          (Utilities|FlowControl|Delay (Variables|Platform|GetStopTime))
          (switch Utilities|FlowControl|Switch|SwitchonETimelineDirection _direction
            (:Forward
              (CallFunction|ReversePlatformMove))
            (:Backward
              (CallFunction|PlayPlatformMove))))))
    (else
      (Timeline|PlatformMovementTimeLine Reverse))))

(event EventBeginPlay
  ;[1 1 1] Play the timeline if it's set to auto play
  (if (Variables|Platform|GetAutoPlay)
    (CallFunction|PlayPlatformMove)))

(fn ConstructionScript
  (bind _destination (Variables|Platform|GetDestination))
  ;[1 1 1] Save the start position
  (Variables|Platform|SetStartTransform (Transformation|GetWorldTransform (Variables|Default|GetPlatformRoot)))
  ;[1 1 1] Set play rate of timeline
  (Components|Timeline|SetPlayRate (Variables|Default|GetPlatformMovementTimeLine) (/ 1.0 (Variables|Platform|GetMoveTime)))
  ;[1 1 1] Preview mesh
  (Transformation|SetRelativeLocationAndRotation (Variables|Default|GetPreviewMesh) (.location _destination) (.rotation _destination) false false))

(fn SetAutoPlay
  (params (AutoPlay :type Boolean))
  (Variables|Platform|SetAutoPlay AutoPlay))