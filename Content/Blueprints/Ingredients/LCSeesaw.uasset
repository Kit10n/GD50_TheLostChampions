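; Seesaw ingredient that catapults characters when an actor lands fast enough on its raised end.
; End trigger overlaps check downward velocity, then play or reverse a timeline that tilts the board, with play rate set at construction.
; When the tilt finishes, characters overlapping the rising end are launched upward and horizontally toward the board's center, and a launch event dispatcher fires.
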(event OnComponentBeginOverlap(SeesawBoardFrontTrigger)
  (params (OtherActor :type Actor%20Object%20Reference) (OtherComp :type Primitive%20Component%20Object%20Reference) (OtherBodyIndex :type Integer) (bFromSweep :type Boolean) (SweepResult :type Hit%20Result%20Structure%20%28by%20ref%29))
  ;[1 1 1] Overlap events
  (Utilities|IsActorZVelocityThreshold OtherActor
    (:True
      (if (not (Variables|Seesaw|GetSeesawFrontDown))
        (CallFunction|ReverseSeesawMoveAnimation)))))

(event OnComponentBeginOverlap(SeesawBoardBackTrigger)
  (params (OtherActor :type Actor%20Object%20Reference) (OtherComp :type Primitive%20Component%20Object%20Reference) (OtherBodyIndex :type Integer) (bFromSweep :type Boolean) (SweepResult :type Hit%20Result%20Structure%20%28by%20ref%29))
  ;[1 1 1] Overlap events
  (Utilities|IsActorZVelocityThreshold OtherActor
    (:True
      (if (Variables|Seesaw|GetSeesawFrontDown)
        (CallFunction|PlaySeesawMoveAnimation)))))

(event Custom|ReverseSeesawMoveAnimation
  (bind _horrizontallaunchforce (Variables|Seesaw|GetHorrizontalLaunchForce))
  ;[1 1 1] Comment
  (if (not (Variables|Seesaw|GetIsMoving))
    (Variables|Seesaw|SetIsMoving true)
    (bind (_direction _0_1) (Timeline|SeesawMoveTimeline ReverseFromEnd)
      (:Update
        (Transformation|SetRelativeRotation (Variables|Default|GetSeesawBoard) (Math|Rotator|Lerp(Rotator) "-20.000000,0.000000, 0" "20.000000,0.000000,0.000000" _0_1 true) false false))
      (:Finished
        (switch Utilities|FlowControl|Switch|SwitchonETimelineDirection _direction
          (:Forward
            (Variables|Seesaw|SetSeesawFrontDown false))
          (:Backward
            (Variables|Seesaw|SetSeesawFrontDown true)))
        (Variables|Seesaw|SetIsMoving false)
        (Utilities|Array|Clear (Variables|Seesaw|GetLaunchedCharacters))
        ;[1 1 1] Comment
        (for _array_element (Collision|GetOverlappingActors (Utilities|Select :Index _direction :Forward (Variables|Default|GetSeesawBoardFrontTrigger) :Backward (Variables|Default|GetSeesawBoardBackTrigger)) 0 :!class /Script/Engine.PrimitiveComponent)
          (bind _aslccharacter_base (Utilities|Casting|CastToLCCharacterBase _array_element))
          (Utilities|Array|AddUnique (Variables|Seesaw|GetLaunchedCharacters) _aslccharacter_base)
          (Character|LaunchCharacter _aslccharacter_base (Math|Vector|MakeVector (.x (* (Math|Vector|GetForwardVector (Math|Rotator|FindLookatRotation (Utilities|Select :Index _direction :Forward (Transformation|GetWorldLocation (Variables|Default|GetSeesawBoardFrontTrigger)) :Backward (Transformation|GetWorldLocation (Variables|Default|GetSeesawBoardBackTrigger))) (Transformation|GetWorldLocation (Variables|Default|GetSeesawBoard)))) (Math|Vector|MakeVector _horrizontallaunchforce _horrizontallaunchforce 0.0))) (.y (* (Math|Vector|GetForwardVector (Math|Rotator|FindLookatRotation (Utilities|Select :Index _direction :Forward (Transformation|GetWorldLocation (Variables|Default|GetSeesawBoardFrontTrigger)) :Backward (Transformation|GetWorldLocation (Variables|Default|GetSeesawBoardBackTrigger))) (Transformation|GetWorldLocation (Variables|Default|GetSeesawBoard)))) (Math|Vector|MakeVector _horrizontallaunchforce _horrizontallaunchforce 0.0))) (Variables|Seesaw|GetVerticalLaunchForce)) false true))
        (Default|CallOnSeesawLaunched self)))))

(event Custom|PlaySeesawMoveAnimation
  (bind _horrizontallaunchforce (Variables|Seesaw|GetHorrizontalLaunchForce))
  ;[1 1 1] Comment
  (if (not (Variables|Seesaw|GetIsMoving))
    (Variables|Seesaw|SetIsMoving true)
    (bind (_direction _0_1) (Timeline|SeesawMoveTimeline PlayFromStart)
      (:Update
        (Transformation|SetRelativeRotation (Variables|Default|GetSeesawBoard) (Math|Rotator|Lerp(Rotator) "-20.000000,0.000000, 0" "20.000000,0.000000,0.000000" _0_1 true) false false))
      (:Finished
        (switch Utilities|FlowControl|Switch|SwitchonETimelineDirection _direction
          (:Forward
            (Variables|Seesaw|SetSeesawFrontDown false))
          (:Backward
            (Variables|Seesaw|SetSeesawFrontDown true)))
        (Variables|Seesaw|SetIsMoving false)
        (Utilities|Array|Clear (Variables|Seesaw|GetLaunchedCharacters))
        ;[1 1 1] Comment
        (for _array_element (Collision|GetOverlappingActors (Utilities|Select :Index _direction :Forward (Variables|Default|GetSeesawBoardFrontTrigger) :Backward (Variables|Default|GetSeesawBoardBackTrigger)) 0 :!class /Script/Engine.PrimitiveComponent)
          (bind _aslccharacter_base (Utilities|Casting|CastToLCCharacterBase _array_element))
          (Utilities|Array|AddUnique (Variables|Seesaw|GetLaunchedCharacters) _aslccharacter_base)
          (Character|LaunchCharacter _aslccharacter_base (Math|Vector|MakeVector (.x (* (Math|Vector|GetForwardVector (Math|Rotator|FindLookatRotation (Utilities|Select :Index _direction :Forward (Transformation|GetWorldLocation (Variables|Default|GetSeesawBoardFrontTrigger)) :Backward (Transformation|GetWorldLocation (Variables|Default|GetSeesawBoardBackTrigger))) (Transformation|GetWorldLocation (Variables|Default|GetSeesawBoard)))) (Math|Vector|MakeVector _horrizontallaunchforce _horrizontallaunchforce 0.0))) (.y (* (Math|Vector|GetForwardVector (Math|Rotator|FindLookatRotation (Utilities|Select :Index _direction :Forward (Transformation|GetWorldLocation (Variables|Default|GetSeesawBoardFrontTrigger)) :Backward (Transformation|GetWorldLocation (Variables|Default|GetSeesawBoardBackTrigger))) (Transformation|GetWorldLocation (Variables|Default|GetSeesawBoard)))) (Math|Vector|MakeVector _horrizontallaunchforce _horrizontallaunchforce 0.0))) (Variables|Seesaw|GetVerticalLaunchForce)) false true))
        (Default|CallOnSeesawLaunched self)))))

(fn ConstructionScript
  ;[1 1 1] Set the play rate of the time line
  (Components|Timeline|SetPlayRate (Variables|Default|GetSeesawMoveTimeline) (Variables|Seesaw|GetSeesawMovePlayRate)))