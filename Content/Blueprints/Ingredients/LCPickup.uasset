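; LCPickup is a collectible potion, coin or gem that player characters collect on overlap.
; The construction script picks the mesh and bobbing/spin endpoints from PickupType for a timeline animation with no wired input.
; PickedUp heals through negative damage or adds coins or a gem to LCPlayerState.
; It then fires OnPickupAcquired and destroys itself, but potions stay when health is full.
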(event OnComponentBeginOverlap(PickupCollision)
  (params (OtherActor :type Actor%20Object%20Reference) (OtherComp :type Primitive%20Component%20Object%20Reference) (OtherBodyIndex :type Integer) (bFromSweep :type Boolean) (SweepResult :type Hit%20Result%20Structure%20%28by%20ref%29))
  ;[1 1 1] Pickup
  (bind _aslccharacter_base (Utilities|Casting|CastToLCCharacterBase OtherActor))
  (if (Variables|/Game/Blueprints/Character/LCCharacterBase.LCCharacterBase_C|GetIsPlayer _aslccharacter_base)
    (Variables|Pickup|SetCharacter _aslccharacter_base)
    (Pickup|PickedUp)))

(fn ConstructionScript
  ;[1 1 1] Mesh
  (Components|StaticMesh|SetStaticMesh (Variables|Default|GetPickupMesh) (Utilities|Select :Index (Variables|Pickup|GetPickupType) :NewEnumerator0 "/Game/Props/Loot/Meshes/PropLoot_PotionMinor_Red.PropLoot_PotionMinor_Red" :NewEnumerator1 "/Game/Props/Loot/Meshes/PropLoot_Coin04.PropLoot_Coin04" :NewEnumerator2 "/Game/Props/Loot/Meshes/PropLoot_Gem_Sapphire.PropLoot_Gem_Sapphire"))
  ;[1 1 1] Set play rate
  (Components|Timeline|SetPlayRate (Variables|Default|GetPickupBobbingTimeline) (Variables|Pickup|GetBobbingPlayRate))
  ;[1 1 1] Position
  (Variables|Pickup|SetBobbingStartPos (Utilities|Select :Index (Variables|Pickup|GetPickupType) :NewEnumerator0 "0,0,30.000000" :NewEnumerator1 "0,0,50.000000" :NewEnumerator2 "0,0,30.000000"))
  (Variables|Pickup|SetBobbingEndPos (Utilities|Select :Index (Variables|Pickup|GetPickupType) :NewEnumerator0 "0,0,70.000000" :NewEnumerator1 "0,0,90.000000" :NewEnumerator2 "0,0,70.000000"))
  ;[1 1 1] Rotation
  (Variables|Pickup|SetBobbingStartRot (Utilities|Select :Index (Variables|Pickup|GetPickupType) :NewEnumerator0 "0.000000,0,0" :NewEnumerator1 "90.000000,0,0" :NewEnumerator2 "0.000000,0,0"))
  (Variables|Pickup|SetBobbingEndRot (Utilities|Select :Index (Variables|Pickup|GetPickupType) :NewEnumerator0 "0.000000,359.000000,0" :NewEnumerator1 "90.000000,359.000000,0" :NewEnumerator2 "0.000000,359.000000,0")))

(fn PickedUp
  (switch Utilities|FlowControl|Switch|SwitchonEnum_PickupType (Variables|Pickup|GetPickupType)
    (:NewEnumerator0
      ;[1 1 1] Potion
      (if (< (Variables|/Game/Blueprints/Character/LCCharacterBase.LCCharacterBase_C|GetHealth (Variables|Pickup|GetCharacter)) (Variables|/Game/Blueprints/Character/LCCharacterBase.LCCharacterBase_C|GetHealthMax (Variables|Pickup|GetCharacter)))
        (Game|Damage|ApplyDamage (Variables|Pickup|GetCharacter) (* (Variables|Pickup|GetHealAmount) -1.0) 0 0)
        (else
          (return))))
    (:NewEnumerator1
      ;[1 1 1] Coin
      (Default|AddCoins (.AsLCPlayer%20State (Utilities|Casting|CastToLCPlayerState (Variables|/Script/Engine.Pawn|GetPlayerState (Variables|Pickup|GetCharacter)))) (Variables|Pickup|GetCoinAmount)))
    (:NewEnumerator2
      ;[1 1 1] Add gem
      (Default|AddGem (.AsLCPlayer%20State (Utilities|Casting|CastToLCPlayerState (Variables|/Script/Engine.Pawn|GetPlayerState (Variables|Pickup|GetCharacter)))))))
  ;[1 1 1] Destroy the actor
  (Default|CallOnPickupAcquired self)
  (Actor|DestroyActor)
  (return))