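; Crumbling platform that shakes, shatters and respawns after an LCCharacterBase hits it from above.
; A hit starts a delayed shake-and-sway timeline, then heavy damage breaks the destructible mesh and a box overlap launches characters still on top.
; SpawnNewRock replaces the component at begin play and after each break, scaling it up before re-arming.
; Dispatchers report crumble, destruction and respawn; the construction script derives timeline play rates from durations.
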(event Custom|PlaySpawnNewRockAnimation
  ;[1 1 1] Spawn animation
  (bind _0_1 (Timeline|SpawnNewRockTimeline PlayFromStart)
    (:Update
      (Transformation|SetWorldScale3D (Variables|Default|GetDMCrumblingRock) (Math|Vector|Lerp(Vector) "0.001000,0.001000,0.001000" "1.000000,1.000000,1.000000" _0_1)))
    (:Finished
      (Variables|Platform|SetIsCrumbling false))))

(event Custom|EventHit
  (params (OtherActor :type Actor%20Object%20Reference) (OtherComp :type Primitive%20Component%20Object%20Reference) (NormalImpulse :type Vector) (Hit :type Hit%20Result%20Structure%20%28by%20ref%29))
  (bind _dmcrumblingrock (Variables|Default|GetDMCrumblingRock))
  ;[1 1 1] Hit events
  (bind _aslccharacter_base (Utilities|Casting|CastToLCCharacterBase OtherActor))
  (if (> (.z (Transformation|GetActorLocation _aslccharacter_base)) (.z (Transformation|GetActorLocation)))
    ;[1 1 1] Start the timer
    (if (not (Variables|Platform|GetIsCrumbling))
      (Variables|Platform|SetCharacterCauser _aslccharacter_base)
      (Variables|Platform|SetIsCrumbling true)
      (Utilities|FlowControl|Delay (Variables|Platform|GetCrumbleDelay))
      (Default|CallOnCrumbleStarted self (Variables|Platform|GetCharacterCauser))
      ;[1 1 1] Shaking and swaing before exploding
      (bind (_direction _0_1 _shaking _swaying) (Timeline|CrumbleTimeline PlayFromStart)
        (:Update
          (Transformation|SetRelativeLocationAndRotation (Variables|Default|GetDMCrumblingRock) (* _shaking 15.0) (Math|Rotator|MakeRotator (.X (Math|Vector|BreakVector (* _swaying 5.0))) (.Y (Math|Vector|BreakVector (* _swaying 5.0))) (.Z (Math|Vector|BreakVector (* _swaying 5.0)))) false false))
        (:Finished
          ;[1 1 1] Destroy rock after slight delay
          (Utilities|FlowControl|Delay (Variables|Platform|GetDestroyPauseDelay))
          (Game|Damage|ApplyDamage _dmcrumblingrock 1e+03 (Transformation|GetWorldLocation _dmcrumblingrock) (Math|Vector|GetUpVector _dmcrumblingrock) (Variables|Platform|GetExplodeImpulseStrength))
          (Default|CallOnPlatformDestroyed self (Variables|Platform|GetCharacterCauser))
          ;[1 1 1] Launch any characters that might be still on the platform
          (bind _outactors (Class|KismetSystemLibrary|BoxOverlapActorsNEW (+ (Transformation|GetActorLocation) "0, 0,50.000000") "100.000000,100.000000,10.000000" (Utilities|Array|MakeArray "ObjectTypeQuery3")))
          (for _array_element _outactors
            (bind _aslccharacter_base_2 (Utilities|Casting|CastToLCCharacterBase _array_element))
            (Character|LaunchCharacter _aslccharacter_base_2 (Variables|Platform|GetLaunchAmount) false true))
          ;[1 1 1] Respawn another rock
          (Utilities|FlowControl|Delay (Variables|Platform|GetRespawnDelay))
          (Platform|SpawnNewRock))))))

(event Custom|AssignNewRockDMHitEvents
  (params (NewDestructibleMesh :type Destructible%20Component%20Object%20Reference))
  ;[1 1 1] Hit events
  (Collision|AssignOnComponentHit NewDestructibleMesh (delegate Custom|EventHit)))

(event EventBeginPlay
  ;[1 1 1] Spawn a rock at begin play
  (Platform|SpawnNewRock))

(fn ConstructionScript
  ;[1 1 1] Timeline
  (Components|Timeline|SetPlayRate (Variables|Default|GetCrumbleTimeline) (/ 1.0 (Variables|Platform|GetCrumbleAnimLength)))
  (Components|Timeline|SetPlayRate (Variables|Default|GetSpawnNewRockTimeline) (/ 1.0 (Variables|Platform|GetSpawnRockAnimLength)))
  (Components|Timeline|SetPlayRate (Variables|Default|GetAmbientMovementTimeline) (/ 1.0 (Variables|Platform|GetAmbientMovementLength))))

(fn SpawnNewRock
  ;[1 1 1] Clean up the old mesh
  (Utilities|IsValid (Variables|Default|GetDMCrumblingRock)
    (:Is%20Valid
      (Components|DestroyComponent (Variables|Default|GetDMCrumblingRock)))
    (:Is%20Not%20Valid
      _))
  ;[1 1 1] Spawn new mesh
  (bind _returnvalue (AddComponent|AddDestructibleComponent false (Math|Transform|MakeTransform "0, 0, 0")))
  (Variables|Default|SetDMCrumblingRock _returnvalue)
  (Variables|/Script/Engine.DestructibleComponent|SetLargeChunkThreshold (Variables|Default|GetDMCrumblingRock) 5e+04)
  (Collision|SetCollisionResponsetoChannel (Variables|Default|GetDMCrumblingRock) "ECC_Camera" "ECR_Ignore")
  (CallFunction|PlaySpawnNewRockAnimation)
  (CallFunction|AssignNewRockDMHitEvents (Variables|Default|GetDMCrumblingRock))
  (Default|CallOnPlatformRespawned self)
  (return (Variables|Default|GetDMCrumblingRock)))