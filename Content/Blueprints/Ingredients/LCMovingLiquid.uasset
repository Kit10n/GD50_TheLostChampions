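; LCMovingLiquid is a configurable water or lava surface that acts as a hazard for overlapping actors.
; The construction script builds a dynamic material from the chosen liquid type, scales the plane and applies user settings for flow speed, liquid scale, displacement and tessellation.
; Overlapping the death collision applies very high damage, typed as drowning for water or lava for lava.
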(event OnComponentBeginOverlap(LiquidDeathCollision)
  (params (OtherActor :type Actor%20Object%20Reference) (OtherComp :type Primitive%20Component%20Object%20Reference) (OtherBodyIndex :type Integer) (bFromSweep :type Boolean) (SweepResult :type Hit%20Result%20Structure%20%28by%20ref%29))
  (Game|Damage|ApplyDamage OtherActor 1e+03 0 self (Utilities|Select :Index (Variables|MovingLiquid|GetLiquidType) :NewEnumerator0 "/Game/Blueprints/Character/LCDmgType_Drown.LCDmgType_Drown_C" :NewEnumerator1 "/Game/Blueprints/Character/LCDmgType_Drown.LCDmgType_Drown_C" :NewEnumerator2 "/Game/Blueprints/Character/LCDmgType_LAva.LCDmgType_Lava_C" :NewEnumerator3 "/Game/Blueprints/Character/LCDmgType_LAva.LCDmgType_Lava_C")))

(fn ConstructionScript
  ;[1 1 1] Create the dynamic material instance so that we may modify it at runtime
  (Variables|MovingLiquid|SetLiquid%20Material (Utilities|Select :Index (Variables|MovingLiquid|GetLiquidType) :NewEnumerator0 "/Game/Environment/MovingLiquid/Materials/Environment_MovingLiquid_WaterClear.Environment_MovingLiquid_WaterClear" :NewEnumerator1 "/Game/Environment/MovingLiquid/Materials/Environment_MovingLiquid_WaterMurky.Environment_MovingLiquid_WaterMurky" :NewEnumerator2 "/Game/Environment/MovingLiquid/Materials/Environment_MovingLiquid_Lava01.Environment_MovingLiquid_Lava01" :NewEnumerator3 "/Game/Environment/MovingLiquid/Materials/Environment_MovingLiquid_Lava02.Environment_MovingLiquid_Lava02"))
  (bind _returnvalue (Rendering|Material|CreateDynamicMaterialInstance (Variables|Default|GetLiquidSurface) 0 (Variables|MovingLiquid|GetLiquid%20Material) :!class /Script/Engine.PrimitiveComponent))
  (Variables|MovingLiquid|SetLiquid%20Material%20Dynamic _returnvalue)
  ;[1 1 1] Set the scale of the plane based off user settings
  (Transformation|SetRelativeScale3D (Variables|Default|GetLiquidSurface) (Math|Vector|MakeVector (Variables|MovingLiquid|GetLiquidScaleX) (Variables|MovingLiquid|GetLiquidScaleY) 1.0))
  ;[1 1 1] Set the properties in the dynamic material insance based off user input
  (Rendering|Material|SetScalarParameterValue (Variables|MovingLiquid|GetLiquid%20Material%20Dynamic) "LiquidSpeed" (Variables|MovingLiquid|GetLiqud%20Speed) :!class /Script/Engine.MaterialInstanceDynamic)
  (Rendering|Material|SetScalarParameterValue (Variables|MovingLiquid|GetLiquid%20Material%20Dynamic) "LiquidScale" (Variables|MovingLiquid|GetOverall%20Liquid%20Scale) :!class /Script/Engine.MaterialInstanceDynamic)
  (Rendering|Material|SetScalarParameterValue (Variables|MovingLiquid|GetLiquid%20Material%20Dynamic) "Displacement" (Variables|MovingLiquid|GetDisplacement) :!class /Script/Engine.MaterialInstanceDynamic)
  (Rendering|Material|SetScalarParameterValue (Variables|MovingLiquid|GetLiquid%20Material%20Dynamic) "Tesselation" (Variables|MovingLiquid|GetTesselation%20Factor) :!class /Script/Engine.MaterialInstanceDynamic))