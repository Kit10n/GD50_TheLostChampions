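; LCMushroom is a bouncy mushroom that launches characters who land on it.
; An overlap with its trigger by a descending LCCharacterBase overrides only vertical launch velocity, plays the bounce animation and notifies through OnCharacterBounced.
; A bounced Druid also plays its ability animation as a dynamic slot montage.
; A timeline stretches and squeezes the mesh relative to the scale captured at construction, and also plays on any damage.
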(event OnComponentBeginOverlap(BounceTrigger)
  (params (OtherActor :type Actor%20Object%20Reference) (OtherComp :type Primitive%20Component%20Object%20Reference) (OtherBodyIndex :type Integer) (bFromSweep :type Boolean) (SweepResult :type Hit%20Result%20Structure%20%28by%20ref%29))
  ;[1 1 1] Bounce!
  (bind _aslccharacter_base (Utilities|Casting|CastToLCCharacterBase OtherActor))
  (if (<= (.Z (Math|Vector|BreakVector (Transformation|GetVelocity _aslccharacter_base))) -1.0)
    (Character|LaunchCharacter _aslccharacter_base (Variables|Mushroom|GetBounceVelocity) false true)
    (CallFunction|PlayBounceAnimation)
    (Default|CallOnCharacterBounced self _aslccharacter_base)
    ;[1 1 1] Play the cool animation for the druid
    (bind _aslccharacter_druid (Utilities|Casting|CastToLCCharacter_Druid _aslccharacter_base))
    (Class|AnimInstance|PlaySlotAnimationasDynamicMontage (Components|SkeletalMesh|GetAnimInstance (Variables|/Script/Engine.Character|GetMesh _aslccharacter_druid)) (Variables|/Game/Blueprints/Character/LCCharacterBase.LCCharacterBase_C|GetAnimAbility01 _aslccharacter_druid) (Variables|/Game/Blueprints/Character/LCCharacterBase.LCCharacterBase_C|GetAnimationSlotName _aslccharacter_druid) (Variables|/Game/Blueprints/Character/LCCharacterBase.LCCharacterBase_C|GetAnim_Ability01BlendInTime _aslccharacter_druid) (Variables|/Game/Blueprints/Character/LCCharacterBase.LCCharacterBase_C|GetAnim_Ability01BlendOutTime _aslccharacter_druid) 1.0 1 -1.0)))

(event Custom|PlayBounceAnimation
  ;[1 1 1] Stretch and squeeze animation
  (bind _scale (Timeline|MushroomBounceTimeline PlayFromStart)
    (:Update
      (Transformation|SetRelativeScale3D (Variables|Default|GetMushroomMesh) (* (Variables|Mushroom|GetStartingScale) _scale)))))

(event Game|Damage|EventAnyDamage
  (params (Damage :type Float%20%28single-precision%29) (DamageType :type Damage%20Type%20Object%20Reference) (InstigatedBy :type Controller%20Object%20Reference) (DamageCauser :type Actor%20Object%20Reference))
  ;[1 1 1] :D
  (CallFunction|PlayBounceAnimation))

(fn ConstructionScript
  ;[1 1 1] Get the starting scale
  (Variables|Mushroom|SetStartingScale (Variables|/Script/Engine.SceneComponent|GetRelativeScale3D (Variables|Default|GetMushroomMesh)))
  ;[1 1 1] Timeline
  (Components|Timeline|SetPlayRate (Variables|Default|GetMushroomBounceTimeline) (Variables|Mushroom|GetMushroomBouncePlayRate)))