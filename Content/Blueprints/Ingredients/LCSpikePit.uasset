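; Resizable spike pit hazard that deals heavy damage to actors entering its collision box.
; The construction script sizes the box from PitSize and tiles spike meshes across it as instanced static meshes spaced by MeshSize.
; On overlap, it damages only actors whose origin is sufficiently above the pit's, then fires OnSpikeDamagedActor with the pit and victim.
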(event OnComponentBeginOverlap(PitCollision)
  (params (OtherActor :type Actor%20Object%20Reference) (OtherComp :type Primitive%20Component%20Object%20Reference) (OtherBodyIndex :type Integer) (bFromSweep :type Boolean) (SweepResult :type Hit%20Result%20Structure%20%28by%20ref%29))
  ;[1 1 1] Damage!
  (if (>= (- (.z (Transformation|GetActorLocation OtherActor)) (.z (Transformation|GetActorLocation))) 6e+01)
    (Game|Damage|ApplyDamage OtherActor 1e+03 0 0)
    (Default|CallOnSpikeDamagedActor self OtherActor)))

(fn ConstructionScript
  (bind _pitsize (Variables|Pit|GetPitSize))
  ;[1 1 1] Set up the box
  (Variables|Pit|SetPitSizeResized (Math|Vector2D|MakeVector2D (Math|Conversions|ToFloat(Integer) (Math|Float|Round (/ (.x _pitsize) 2.0))) (Math|Conversions|ToFloat(Integer) (Math|Float|Round (/ (.y _pitsize) 2.0)))))
  (Components|Box|SetBoxExtent (Variables|Default|GetPitCollision) (Math|Vector|MakeVector (.x (Variables|Pit|GetPitSizeResized)) (.y (Variables|Pit|GetPitSizeResized)) 1e+01) false)
  ;[1 1 1] Create all the meshes
  (for _index (range 0 (Math|Float|Round (* (/ (.y (Variables|Pit|GetPitSizeResized)) (Variables|Pit|GetMeshSize)) 2.0)))
    (for _index_2 (range 0 (Math|Float|Round (* (/ (.x (Variables|Pit|GetPitSizeResized)) (Variables|Pit|GetMeshSize)) 2.0)))
      (Components|InstancedStaticMesh|AddInstance (Variables|Default|GetInstancedStaticMesh) (Math|Transform|MakeTransform (Math|Vector|MakeVector (- (* _index_2 (Variables|Pit|GetMeshSize)) (.x (Variables|Pit|GetPitSizeResized))) (- (* _index (Variables|Pit|GetMeshSize)) (.y (Variables|Pit|GetPitSizeResized))) 0.0))))))