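; LCPortal teleports an overlapping character to a linked destination portal, one trip at a time.
; It disables input, hides the character and moves a coloured sphere along a timeline while the camera focuses on a target point attached to it.
; Capsule overlap tests pick an unoccupied exit arrow, falling back to the first.
; On arrival it moves and reveals the character with smoke, restores input and calls OnPortalUsed.
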(event OnComponentBeginOverlap(PortalCollision)
  (params (OtherActor :type Actor%20Object%20Reference) (OtherComp :type Primitive%20Component%20Object%20Reference) (OtherBodyIndex :type Integer) (bFromSweep :type Boolean) (SweepResult :type Hit%20Result%20Structure%20%28by%20ref%29))
  ;[1 1 1] Overlap event
  (bind _aslccharacter_base (Utilities|Casting|CastToLCCharacterBase OtherActor))
  (Utilities|IsValid (Variables|Teleporter|GetPortalDestination)
    (:Is%20Valid
      (if (not (Variables|Teleporter|GetPortalInUse))
        (Variables|Teleporter|SetPortalInUse true)
        (Variables|Teleporter|SetCharacter _aslccharacter_base)
        (CallFunction|PlaySphereMovementAnim)))))

(event Custom|PlaySphereMovementAnim
  (bind _character (Variables|Teleporter|GetCharacter))
  (bind _character_2 (Variables|Teleporter|GetCharacter))
  (bind _portaldestination (Variables|Teleporter|GetPortalDestination))
  (bind _returnvalue (Pawn|GetController _character_2))
  (bind _returnvalue_2 (Pawn|GetController _character))
  (bind _aslcplayer_controller (Utilities|Casting|CastToLCPlayerController _returnvalue_2))
  (bind _aslcplayer_controller_2 (Utilities|Casting|CastToLCPlayerController _returnvalue))
  ;[1 1 1] Sphere movement
  (Input|DisableInput _aslcplayer_controller_2 _aslcplayer_controller_2)
  (Default|PlayCamtoCharAnimation _aslcplayer_controller_2 (Variables|Teleporter|GetCameraFocus))
  (Rendering|SetVisibility (Variables|Default|GetPortalMovementSphere) true false)
  (Rendering|SetVisibility (Variables|/Script/Engine.Character|GetCapsuleComponent (Variables|Teleporter|GetCharacter)) false true)
  (Components|Activation|Activate (Variables|Default|GetPS_TeleporterSphere) true)
  ;[1 1 1] Find correct destination
  (Variables|Default|SetChosenPortalDestinationArrow (Teleporter|ChoosePortalDestination (Utilities|Array|MakeArray (Variables|LCPortal_C|GetPortalSpawnArrow02 _portaldestination) (Variables|LCPortal_C|GetPortalSpawnArrow01 _portaldestination) (Variables|LCPortal_C|GetPortalSpawnArrow03 _portaldestination))))
  (bind _0_1 (Timeline|SphereMovementTimeline PlayFromStart)
    (:Update
      ;[1 1 1] Movement
      (Transformation|SetWorldLocation (Variables|Default|GetPortalMovementSphere) (Math|Vector|Lerp(Vector) (Transformation|GetWorldLocation (Variables|Default|GetPS_Portal)) (Transformation|GetWorldLocation (Variables|Default|GetChosenPortalDestinationArrow)) _0_1) false false))
    (:Finished
      ;[1 1 1] Clean up
      (Variables|Teleporter|SetPortalInUse false)
      (Rendering|SetVisibility (Variables|Default|GetPortalMovementSphere) false false)
      (Transformation|SetActorLocationAndRotation (Variables|Teleporter|GetCharacter) (Transformation|GetWorldLocation (Variables|Default|GetChosenPortalDestinationArrow)) (Math|Rotator|MakeRotator 0.0 0.0 (.Yaw (Math|Rotator|BreakRotator (Transformation|GetWorldRotation (Variables|Default|GetChosenPortalDestinationArrow))))))
      (Effects|SpawnEmitteratLocation "/Game/Effects/Particles/Systems/DeadSmoke_Particle.DeadSmoke_Particle" (Transformation|GetWorldLocation (Variables|Default|GetChosenPortalDestinationArrow)) (Math|Rotator|MakeRotator 0.0 0.0 (.Yaw (Math|Rotator|BreakRotator (Transformation|GetWorldRotation (Variables|Default|GetChosenPortalDestinationArrow))))))
      (Rendering|SetVisibility (Variables|/Script/Engine.Character|GetCapsuleComponent (Variables|Teleporter|GetCharacter)) true true)
      (Components|Timeline|SetPlaybackPosition (Variables|/Game/Blueprints/Character/LCPlayerController.LCPlayerController_C|GetCamToCharTimeline (.AsLCPlayer%20Controller (Utilities|Casting|CastToLCPlayerController (Pawn|GetController (Variables|Teleporter|GetCharacter))))) 1.0 true true)
      (Input|EnableInput _aslcplayer_controller _aslcplayer_controller)
      (Components|Activation|Deactivate (Variables|Default|GetPS_TeleporterSphere))
      (Default|CallOnPortalUsed self (Variables|Teleporter|GetPortalDestination) (Variables|Teleporter|GetCharacter)))))

(event EventBeginPlay
  ;[1 1 1] Create a dummy actor and attach it to the sphere
  (bind _returnvalue (Game|SpawnActorfromClass "/Script/Engine.TargetPoint" (Transformation|GetWorldTransform (Variables|Default|GetPortalMovementSphere)) "AlwaysSpawn" 0 0))
  (bind _output_get (Variables|Teleporter|SetCameraFocus _returnvalue))
  (Class|Actor|AttachRootComponentto _output_get (Variables|Default|GetPortalMovementSphere) "None" "SnapToTargetIncludingScale" true))

(fn ConstructionScript
  ;[1 1 1] Create the DMI and initially set the colours
  (bind _returnvalue (Rendering|Material|CreateDynamicMaterialInstance (Variables|Default|GetPortalMovementSphere) 0 0 :!class /Script/Engine.PrimitiveComponent))
  (Variables|Teleporter|SetSphereDMI _returnvalue)
  (Teleporter|SetParticleandSphereColour (Variables|Teleporter|GetPortalColour))
  ;[1 1 1] Set play rate
  (Components|Timeline|SetPlayRate (Variables|Default|GetSphereMovementTimeline) (Variables|Teleporter|GetSphereMovementPlayRate)))

(fn SetParticleandSphereColour
  (params (Colour :type Linear%20Color%20Structure))
  ;[1 1 1] Init
  (LocalVariables|SetColourLocal Colour)
  ;[1 1 1] Particle and material colour
  (Effects|Components|ParticleSystem|SetColorParameter (Variables|Default|GetPS_Portal) "PortalColor" (LocalVariables|GetColourLocal))
  (Effects|Components|ParticleSystem|SetColorParameter (Variables|Default|GetPS_TeleporterSphere) "PortalColor" (LocalVariables|GetColourLocal))
  (Rendering|Material|SetVectorParameterValue (Variables|Teleporter|GetSphereDMI) "PortalColor" (LocalVariables|GetColourLocal) :!class /Script/Engine.MaterialInstanceDynamic)
  (return))

(fn ChoosePortalDestination
  (params (SceneComponents :type Array%20of%20Scene%20Component%20Object%20References))
  (LocalVariables|SetSceneComponentsLocal SceneComponents)
  (bind _array_element (Utilities|Array|ForEachLoopwithBreak (LocalVariables|GetSceneComponentsLocal) :!label _label)
    (:LoopBody
      (LocalVariables|SetPlayerOccupiedDestinationLocal false)
      (bind _outactors (Class|KismetSystemLibrary|CapsuleOverlapActorsNEW (Transformation|GetWorldLocation _array_element) 25.0 45.0 (Utilities|Array|MakeArray "ObjectTypeQuery3")))
      (for _array_element_2 _outactors
        (Utilities|Casting|CastToLCCharacterBase _array_element_2)
        (LocalVariables|SetPlayerOccupiedDestinationLocal true)
        (Development|PrintString "Hello"))
      (if (not (LocalVariables|GetPlayerOccupiedDestinationLocal))
        (LocalVariables|SetChosenDestinationLocal _array_element)
        (Development|PrintString "Chosen")
        (goto _label Break)))
    (:Completed
      (Utilities|IsValid (LocalVariables|GetChosenDestinationLocal)
        (:Is%20Valid
          _)
        (:Is%20Not%20Valid
          (LocalVariables|SetChosenDestinationLocal (Utilities|Array|Get(acopy) (LocalVariables|GetSceneComponentsLocal)))))
      (return (LocalVariables|GetChosenDestinationLocal)))))

(fn SetPortalDestination
  (params (PortalDestination :type LC%20Portal%20Object%20Reference))
  (Variables|Teleporter|SetPortalDestination PortalDestination))