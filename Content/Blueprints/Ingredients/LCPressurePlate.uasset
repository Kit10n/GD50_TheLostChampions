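; Pressure plate that sinks while characters stand on it and announces when it is activated or deactivated.
; An overlap counter, filtered to LCCharacterBase actors, plays a movement timeline for the first one on and reverses it for the last one off.
; Activated and deactivated calls fire when the timeline finishes and the down state changes.
; BeginPlay also checks existing overlaps, jumping the timeline ahead for plates already occupied.
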(event OnComponentBeginOverlap(PressurePlateCollision)
  (params (OtherActor :type Actor%20Object%20Reference) (OtherComp :type Primitive%20Component%20Object%20Reference) (OtherBodyIndex :type Integer) (bFromSweep :type Boolean) (SweepResult :type Hit%20Result%20Structure%20%28by%20ref%29))
  ;[1 1 1] When a character or pushable block overlaps us
  (bind _foundvalidoverlap (PressurePlate|CheckValidOverlappingActors OtherActor OtherComp))
  (if _foundvalidoverlap
    ;[1 1 1] Only activate/detactive if it's the first/last person on/off the switch
    (bind _output_get (Variables|PressurePlate|SetNumberOfOverlapping (+ (Variables|PressurePlate|GetNumberOfOverlapping) 1)))
    (if (== _output_get 1)
      ;[1 1 1] Play the movement animation
      (bind (_direction _0_1) (Timeline|PressurePlateTimeline Play)
        (:Update
          (Transformation|SetRelativeLocation (Variables|Default|GetPressurePlate) (Math|Vector|MakeVector 0.0 0.0 (Math|Float|Lerp 0.0 (Variables|PressurePlate|GetPressurePlateAnimDistance) _0_1)) false false))
        (:Finished
          ;[1 1 1] Let everyone know what we're up to
          (switch Utilities|FlowControl|Switch|SwitchonETimelineDirection _direction
            (:Forward
              (if (not (Variables|PressurePlate|GetIsPressurePlateDown))
                (Variables|PressurePlate|SetIsPressurePlateDown true)
                (Default|CallOnPressurePlateActivated self)
                (else
                  (Variables|PressurePlate|SetIsPressurePlateDown true))))
            (:Backward
              (if (Variables|PressurePlate|GetIsPressurePlateDown)
                (Variables|PressurePlate|SetIsPressurePlateDown false)
                (Default|CallOnPressurePlateDeactivated self)
                (else
                  (Variables|PressurePlate|SetIsPressurePlateDown false))))))))))

(event OnComponentEndOverlap(PressurePlateCollision)
  (params (OtherActor :type Actor%20Object%20Reference) (OtherComp :type Primitive%20Component%20Object%20Reference) (OtherBodyIndex :type Integer))
  ;[1 1 1] When a character or pushable block overlaps us
  (bind _foundvalidoverlap (PressurePlate|CheckValidOverlappingActors OtherActor OtherComp))
  (if _foundvalidoverlap
    ;[1 1 1] Only activate/detactive if it's the first/last person on/off the switch
    (bind _output_get (Variables|PressurePlate|SetNumberOfOverlapping (- (Variables|PressurePlate|GetNumberOfOverlapping) 1)))
    (if (== _output_get 0)
      ;[1 1 1] Play the movement animation
      (bind (_direction _0_1) (Timeline|PressurePlateTimeline Reverse)
        (:Update
          (Transformation|SetRelativeLocation (Variables|Default|GetPressurePlate) (Math|Vector|MakeVector 0.0 0.0 (Math|Float|Lerp 0.0 (Variables|PressurePlate|GetPressurePlateAnimDistance) _0_1)) false false))
        (:Finished
          ;[1 1 1] Let everyone know what we're up to
          (switch Utilities|FlowControl|Switch|SwitchonETimelineDirection _direction
            (:Forward
              (if (not (Variables|PressurePlate|GetIsPressurePlateDown))
                (Variables|PressurePlate|SetIsPressurePlateDown true)
                (Default|CallOnPressurePlateActivated self)
                (else
                  (Variables|PressurePlate|SetIsPressurePlateDown true))))
            (:Backward
              (if (Variables|PressurePlate|GetIsPressurePlateDown)
                (Variables|PressurePlate|SetIsPressurePlateDown false)
                (Default|CallOnPressurePlateDeactivated self)
                (else
                  (Variables|PressurePlate|SetIsPressurePlateDown false))))))))))

(event EventBeginPlay
  ;[1 1 1] Check if there's any overlapping actors at begin play
  (for _array_element (Collision|GetOverlappingActors (Variables|Default|GetPressurePlateCollision) 0 :!class /Script/Engine.PrimitiveComponent)
    (for _array_element_2 0
      (bind _foundvalidoverlap (PressurePlate|CheckValidOverlappingActors _array_element _array_element_2))
      (if _foundvalidoverlap
        (Components|Timeline|SetPlaybackPosition (Variables|Default|GetPressurePlateTimeline) 1.0 true true)
        ;[1 1 1] Only activate/detactive if it's the first/last person on/off the switch
        (bind _output_get (Variables|PressurePlate|SetNumberOfOverlapping (+ (Variables|PressurePlate|GetNumberOfOverlapping) 1)))
        (if (== _output_get 1)
          ;[1 1 1] Play the movement animation
          (bind (_direction _0_1) (Timeline|PressurePlateTimeline Play)
            (:Update
              (Transformation|SetRelativeLocation (Variables|Default|GetPressurePlate) (Math|Vector|MakeVector 0.0 0.0 (Math|Float|Lerp 0.0 (Variables|PressurePlate|GetPressurePlateAnimDistance) _0_1)) false false))
            (:Finished
              ;[1 1 1] Let everyone know what we're up to
              (switch Utilities|FlowControl|Switch|SwitchonETimelineDirection _direction
                (:Forward
                  (if (not (Variables|PressurePlate|GetIsPressurePlateDown))
                    (Variables|PressurePlate|SetIsPressurePlateDown true)
                    (Default|CallOnPressurePlateActivated self)
                    (else
                      (Variables|PressurePlate|SetIsPressurePlateDown true))))
                (:Backward
                  (if (Variables|PressurePlate|GetIsPressurePlateDown)
                    (Variables|PressurePlate|SetIsPressurePlateDown false)
                    (Default|CallOnPressurePlateDeactivated self)
                    (else
                      (Variables|PressurePlate|SetIsPressurePlateDown false))))))))))))

(fn ConstructionScript
  ;[1 1 1] Set the speed of the animation timeline
  (Components|Timeline|SetPlayRate (Variables|Default|GetPressurePlateTimeline) (Variables|PressurePlate|GetPressurePlatePlayRate)))

(fn CheckValidOverlappingActors
  (params (Actor :type Object%20Object%20Reference) (Component :type Primitive%20Component%20Object%20Reference))
  ;[1 1 1] Init vars
  (LocalVariables|SetActorLocal Actor)
  (LocalVariables|SetComponentLocal Component)
  ;[1 1 1] Check if it's an object we care about
  (Utilities|Casting|CastToLCCharacterBase (LocalVariables|GetActorLocal)
    (:then
      (LocalVariables|SetFoundValidOverlapLocal true))
    (:CastFailed
      (LocalVariables|SetFoundValidOverlapLocal false)))
  ;[1 1 1] Return
  (return (LocalVariables|GetFoundValidOverlapLocal)))