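; LCOrb is a switch orb that toggles between on and off states when it takes damage.
; Each hit flips the state, recolours the orb and broadcasts OnOrbSwitched with the new state, damage causer and instigator.
; A DoOnce reset by a short delay acts as a cooldown between toggles.
; A timeline drives a hit flash on a dynamic material instance created in the construction script.
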(event Custom|PlayHitFlashAnimation
  ;[1 1 1] Hit flash anim
  (bind _hitflash (Timeline|HitFlashTimeline PlayFromStart)
    (:Update
      (Rendering|Material|SetScalarParameterValue (Variables|Orb|GetOrbDMI) "HitFlash" _hitflash :!class /Script/Engine.MaterialInstanceDynamic))))

(event Game|Damage|EventAnyDamage
  (params (Damage :type Float%20%28single-precision%29) (DamageType :type Damage%20Type%20Object%20Reference) (InstigatedBy :type Controller%20Object%20Reference) (DamageCauser :type Actor%20Object%20Reference))
  ;[1 1 1] Toggle the orb based on damage
  (Variables|Orb|SetInstigatedBy InstigatedBy)
  (Variables|Orb|SetCausedBy DamageCauser)
  (Utilities|FlowControl|DoOnce false :!label _label
    (:Completed
      (Utilities|FlowControl|Sequence
        (:then_0
          (bind _isa (Utilities|FlowControl|FlipFlop)
            (:A
              _)
            (:B
              _))
          (Variables|Orb|SetIsOrbOn _isa)
          (Rendering|Material|SetVectorParameterValue (Variables|Orb|GetOrbDMI) "OrbColour" (select (Variables|Orb|GetIsOrbOn) (Variables|Orb|GetOnColour) (Variables|Orb|GetOffColour)) :!class /Script/Engine.MaterialInstanceDynamic)
          (Variables|Orb|SetOrbState (select (Variables|Orb|GetIsOrbOn) "NewEnumerator0" "NewEnumerator1"))
          (Default|CallOnOrbSwitched self (Variables|Orb|GetOrbState) (Variables|Orb|GetCausedBy) (Variables|Orb|GetInstigatedBy))
          (CallFunction|PlayHitFlashAnimation))
        (:then_1
          (Utilities|FlowControl|Delay 0.5)
          (goto _label Reset))))))

(fn ConstructionScript
  ;[1 1 1] Dynamic material instance
  (bind _returnvalue (Rendering|Material|CreateDynamicMaterialInstance (Variables|Default|GetOrbMesh) 0 0 :!class /Script/Engine.PrimitiveComponent))
  (Variables|Orb|SetOrbDMI _returnvalue)
  (Components|Timeline|SetPlayRate (Variables|Default|GetHitFlashTimeline) (Variables|Orb|GetHitFlashPlayRate)))