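; LCAISpawner is a placeable actor that spawns an AI character of a configurable class at its transform, raised slightly in Z.
; On BeginPlay it destroys its placeholder mesh and spawns immediately if SpawnOnBeginPlay is set.
; SpawnAI ignores collision, then applies the wander setting and initial patrol path to the new LCAIController.
; It stores and returns the character and controller, which GetSpawnedAI also exposes.
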(event EventBeginPlay
  ;[1 1 1] Remove the mesh
  (Components|DestroyComponent (Variables|Default|GetAISpawnerMesh))
  ;[1 1 1] Spawn the AI at the get go if the boolean is set to true
  (if (Variables|Spawner|GetSpawnOnBeginPlay)
    (Spawner|SpawnAI)))

(fn ConstructionScript)

(fn SpawnAI
  (bind _returnvalue (Transformation|GetActorTransform))
  (bind _returnvalue_2 (AI|SpawnAIFromClass (Variables|Spawner|GetSpawnedClass) 0 (+ (.location _returnvalue) "0, 0,45.000000") (.rotation _returnvalue) true))
  (Variables|Spawner|SetSpawnedCharacter (.AsLCCharacter%20Base (Utilities|Casting|CastToLCCharacterBase _returnvalue_2)))
  (bind _output_get (Variables|Spawner|SetSpawnedController (.AsLCAIController (Utilities|Casting|CastToLCAIController (Pawn|GetController (.AsLCCharacter%20Base (Utilities|Casting|CastToLCCharacterBase _returnvalue_2)))))))
  (Default|SetWander _output_get (not (Variables|Spawner|GetDoNotWander)))
  (Default|SetPatrolPath (Variables|Spawner|GetSpawnedController) (Variables|Spawner|GetInitialPatrolPath))
  (return (Variables|Spawner|GetSpawnedCharacter) (Variables|Spawner|GetSpawnedController)))

(fn GetSpawnedAI
  (return (Variables|Spawner|GetSpawnedCharacter) (Variables|Spawner|GetSpawnedController)))