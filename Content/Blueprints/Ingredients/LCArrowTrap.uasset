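; LCArrowTrap is a crossbow trap that fires LCArrow projectiles after a delay, once or repeatedly, optionally starting on BeginPlay.
; Activation sets a timer that spawns each arrow at the ArrowSpawn transform, broadcasts OnProjectileFired and plays a timeline-driven recoil on the crossbow mesh.
; Deactivation clears the timer.
; SetFireDelay only stores the value, leaving any running timer unchanged.
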(event Custom|PlayRecoilAnimation
  (bind _crossbowstartpos (Variables|ArrowTrap|GetCrossbowStartPos))
  ;[1 1 1] Recoil
  (bind _movement (Timeline|RecoilTimeline PlayFromStart)
    (:Update
      (Transformation|SetRelativeLocation (Variables|Default|GetCrossbowMesh) (Math|Vector|Lerp(Vector) _crossbowstartpos (+ _crossbowstartpos "-5.000000, 0, 0") _movement) false false))))

(event Custom|ActivateArrowTrap
  (params (AutomaticFire :type Boolean) (FireDelay :type Float%20%28single-precision%29))
  ;[1 1 1] Activation/deactivation
  (bind _returnvalue (Utilities|Time|SetTimerbyFunctionName 0 "SpawnArrowProjectile" FireDelay AutomaticFire)))

(event Custom|DeactivateArrowTrap
  ;[1 1 1] Activation/deactivation
  (Utilities|Time|ClearandInvalidateTimerbyHandle (stale Custom|ActivateArrowTrap _returnvalue)))

(event EventBeginPlay
  ;[1 1 1] Start firing
  (if (Variables|ArrowTrap|GetSpawnFiring)
    (CallFunction|ActivateArrowTrap (Variables|ArrowTrap|GetAutomaticFiring) (Variables|ArrowTrap|GetFireDelay))))

(fn ConstructionScript
  ;[1 1 1] Get pos
  (Variables|ArrowTrap|SetCrossbowStartPos (Variables|/Script/Engine.SceneComponent|GetRelativeLocation (Variables|Default|GetCrossbowMesh)))
  (Components|Timeline|SetPlayRate (Variables|Default|GetRecoilTimeline) (Variables|ArrowTrap|GetRecoilPlayRate)))

(fn SpawnArrowProjectile
  (bind _returnvalue (Game|SpawnActorfromClass "/Game/Blueprints/Ingredients/LCArrow.LCArrow_C" (Transformation|GetWorldTransform (Variables|Default|GetArrowSpawn)) "AlwaysSpawn" self 0))
  (Default|CallOnProjectileFired self _returnvalue)
  (CallFunction|PlayRecoilAnimation)
  (return))

(fn SetFireDelay
  (params (FireDelay :type Float%20%28single-precision%29))
  (Variables|ArrowTrap|SetFireDelay FireDelay))