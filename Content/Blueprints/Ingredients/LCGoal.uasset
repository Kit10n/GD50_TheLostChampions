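; Level goal that completes the level once the player champions overlapping its collision match the alive count.
; Overlap events track champions in an array and update a scroll widget counter, then a DoOnce calls LevelComplete on the game mode.
; Victory animations play while a timeline turns champions toward VictoryCamera.
; CreateLevelCompleteUI spawns the finished UI before that camera and hides health bars; the scroll bobbing logic is unconnected.
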(event OnComponentBeginOverlap(GoalCollision)
  (params (OtherActor :type Actor%20Object%20Reference) (OtherComp :type Primitive%20Component%20Object%20Reference) (OtherBodyIndex :type Integer) (bFromSweep :type Boolean) (SweepResult :type Hit%20Result%20Structure%20%28by%20ref%29))
  ;[1 1 1] Champions entering and exiting
  (bind _aslccharacter_base (Utilities|Casting|CastToLCCharacterBase OtherActor))
  (if (Variables|/Game/Blueprints/Character/LCCharacterBase.LCCharacterBase_C|GetIsPlayer _aslccharacter_base)
    (Utilities|Array|AddUnique (Variables|Default|GetCharactersArray) _aslccharacter_base)
    (Variables|Default|SetCurrentOverlapAmount (+ (Variables|Default|GetCurrentOverlapAmount) 1))
    (CallFunction|UpdateScrollText)
    (if (== (Variables|Default|GetCurrentOverlapAmount) (Variables|Default|GetCurrentAliveAmount))
      (Utilities|FlowControl|DoOnce false
        (:Completed
          (Default|LevelComplete (.AsLCGame%20Mode (Utilities|Casting|CastToLCGameMode (Game|GetGameMode))))
          (CallFunction|PlayChamptoCamAnimation))))))

(event OnComponentEndOverlap(GoalCollision)
  (params (OtherActor :type Actor%20Object%20Reference) (OtherComp :type Primitive%20Component%20Object%20Reference) (OtherBodyIndex :type Integer))
  ;[1 1 1] Champions entering and exiting
  (bind _aslccharacter_base (Utilities|Casting|CastToLCCharacterBase OtherActor))
  (if (Variables|/Game/Blueprints/Character/LCCharacterBase.LCCharacterBase_C|GetIsPlayer _aslccharacter_base)
    (Utilities|Array|RemoveItem (Variables|Default|GetCharactersArray) _aslccharacter_base)
    (Variables|Default|SetCurrentOverlapAmount (- (Variables|Default|GetCurrentOverlapAmount) 1))
    (CallFunction|UpdateScrollText)))

(event Custom|PlayChampToCamAnimation
  ;[1 1 1] Turn to cam animation
  (for _array_element (Variables|Default|GetCharactersArray)
    (Components|Animation|PlayAnimation (Variables|/Script/Engine.Character|GetMesh _array_element) (Variables|/Game/Blueprints/Character/LCCharacterBase.LCCharacterBase_C|GetAnimVictory _array_element) true))
  (bind _movement (Timeline|ChampionTurnToCamTimeline PlayFromStart)
    (:Update
      (for _array_element_2 (Variables|Default|GetCharactersArray)
        (Utilities|IsValid _array_element_2
          (:Is%20Valid
            (Transformation|SetActorRotation _array_element_2 (Math|Rotator|Lerp(Rotator) (Transformation|GetActorRotation _array_element_2) (Math|Rotator|MakeRotator 0.0 0.0 (.yaw (Math|Rotator|FindLookatRotation (Transformation|GetActorLocation _array_element_2) (Transformation|GetWorldLocation (Variables|Default|GetVictoryCamera))))) _movement true))))))))

(fn ConstructionScript
  ;[1 1 1] Bobbing timeline
  (Variables|Default|SetScrollStartPos (Variables|/Script/Engine.SceneComponent|GetRelativeLocation (Variables|Default|GetScrollMesh)))
  (Components|Timeline|SetPlayRate (Variables|Default|GetScrollBobbingTimeline) (Variables|Default|GetBobbingTimeline))
  (Components|Timeline|SetPlayRate (Variables|Default|GetChampionTurnToCamTimeline) (Variables|Default|GetChampToCamPlayRate)))

(fn UpdateScrollText
  (Rendering|Components|TextRender|SetText (Variables|/Game/UI/UMG/LCUMG_GoalCounter.LCUMG_GoalCounter_C|GetChampionCount (.AsLCUMG%20Goal%20Counter (Utilities|Casting|CastToLCUMG_GoalCounter (UserInterface|GetUserWidgetObject (Variables|Default|GetScrollTextWidget))))) (Utilities|Text|ToText(Integer) (Variables|Default|GetCurrentOverlapAmount)))
  (Rendering|Components|TextRender|SetText (Variables|/Game/UI/UMG/LCUMG_GoalCounter.LCUMG_GoalCounter_C|GetAliveChampionCount (.AsLCUMG%20Goal%20Counter (Utilities|Casting|CastToLCUMG_GoalCounter (UserInterface|GetUserWidgetObject (Variables|Default|GetScrollTextWidget))))) (Utilities|Text|FormatText "/{Alive}" (Utilities|Text|ToText(Integer) (Variables|Default|GetCurrentAliveAmount))))
  (return))

(fn CreateLevelCompleteUI
  (bind _victorycamera (Variables|Default|GetVictoryCamera))
  (bind _returnvalue (Transformation|GetWorldTransform _victorycamera))
  (bind (_location _rotation _scale) (Math|Transform|BreakTransform _returnvalue))
  (bind _returnvalue_2 (Math|Vector|GetForwardVector _rotation))
  (bind _returnvalue_3 (* _returnvalue_2 125.0))
  (bind _returnvalue_4 (+ _location _returnvalue_3))
  (Game|SpawnActorfromClass "/Game/Blueprints/Game/LCLevelFinishedUI.LCLevelFinishedUI_C" (Math|Transform|MakeTransform _returnvalue_4 (Math|Rotator|FindLookatRotation _returnvalue_4 _location) _scale) "AlwaysSpawn" 0 "NewEnumerator0" 0)
  ;[1 1 1] Hide their health bars
  (for _array_element (Variables|Default|GetCharactersArray)
    (Rendering|SetVisibility (Variables|/Game/Blueprints/Character/LCCharacterBase.LCCharacterBase_C|GetHealthBar _array_element) false false)))